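; AR scene actor in which a drone flies in and projects a talking hologram man who delivers a speech, then hints at a clue behind a photo.
; BeginPlay either plays this sequence or hides the drone and shows a hint, depending on DroneState.
; Timelines drive the drone move and hologram scale-up, while gated Perlin noise flickers flare and material.
; A looping timer randomly toggles the material's mouth expression during speech, faking lip movement.
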(event Custom|play
  (bind _returnvalue (Utilities|Time|GetGameTimeinSeconds))
  (bind _returnvalue_2 (* _returnvalue 8.0))
  (bind _returnvalue_3 (Class|KismetMathLibrary|PerlinNoise1D _returnvalue_2))
  (bind _returnvalue_4 (+ _returnvalue_3 0.5))
  (bind _returnvalue_5 (Math|Float|Clamp(Float) _returnvalue_4 0.0 1e+01))
  (bind _returnvalue_6 (/ _returnvalue_5 3.0))
  ;[1 1 1] 在摄像机前展示场景
  (Audio|Components|Audio|Play (Variables|Default|GetSFX_9) 0.0)
  (bind _newtrack_0 (Timeline|Timeline_0 Play)
    (:Update
      (Transformation|SetWorldTransform (Variables|Default|GetdroneRoot) (Math|Transform|Lerp(Transform) (Transformation|GetWorldTransform (Variables|Default|GetScene)) (Transformation|GetWorldTransform (Variables|Default|GetScene1)) _newtrack_0) false false))
    (:Finished
      (Utilities|FlowControl|Delay 1.0)
      (Utilities|FlowControl|Sequence
        (:then_0
          (Utilities|FlowControl|Gate true) ; enters at Open
        )
        (:then_1
          (Utilities|FlowControl|Delay 1.0)
          (Utilities|FlowControl|Sequence
            (:then_0
              (bind _newtrack_0_2 (Timeline|Timeline_1 Play)
                (:Update
                  (Transformation|SetRelativeScale3D (Variables|Default|GetmanRoot) (Math|Vector|MakeVector _newtrack_0_2 _newtrack_0_2 _newtrack_0_2)))))
            (:then_1
              (Utilities|FlowControl|Delay 1.0)
              (Audio|Components|Audio|Play (Variables|Default|Getspeech) 0.0))
            (:then_2
              (Utilities|FlowControl|Delay 1.0)
              ;[1 1 1] 说话动画
              (bind _returnvalue_7 (Utilities|Time|SetTimerbyEvent (delegate Custom|changeExoression) 0.2 true)))
            (:then_3
              (Utilities|FlowControl|Delay 14.0)
              (Transformation|SetRelativeScale3D (Variables|Default|GetmanRoot) "0, 0, 0")
              (bind _returnvalue_8 (UserInterface|CreateWidget "/Game/GameDays/6_0/HintWidget/Bottom_Hint_Widget.Bottom_Hint_Widget_C"))
              (Rendering|Components|TextRender|SetText (Variables|/Game/GameDays/6_0/HintWidget/Bottom_Hint_Widget.Bottom_Hint_Widget_C|GetTextBlock_79 _returnvalue_8) "这幅照片背后时空如果封存了神器的话，会给我留什么线索呢？我仔细观察下...")
              (Variables|Default|SetBottomHintUI _returnvalue_8)
              (UserInterface|Viewport|AddtoViewport _returnvalue_8 0)
              (Transformation|SetRelativeScale3D (Variables|Default|GetflareRoot) "0, 0, 0")
              (Utilities|FlowControl|Sequence
                (:then_0
                  (Rendering|SetVisibility (Variables|Default|Getdrone) false false)
                  (Default|CallHasFinishedHearing))
                (:then_1
                  (Utilities|FlowControl|Gate true) ; enters at Close
                )))))
        (:then_2
          (bind _newtrack_0_3 (Timeline|Timeline_2 Play)
            (:Update
              (Variables|Default|SetflickRate (* _newtrack_0_3 8.0)))))))))

(event Custom|changeExoression
  ;[1 1 1] 说话动画
  (if (Variables|Default|GetopenMouth)
    (Rendering|Material|SetVectorParameterValue :self (Variables|Default|GetdynamicMaterial) :ParameterName "expression" :!class /Script/Engine.MaterialInstanceDynamic)
    (Variables|Default|SetopenMouth false)
    (elif (> (Math|Random|RandomFloatinRange 0.0 1.0) 0.5)
      (Rendering|Material|SetVectorParameterValue (Variables|Default|GetdynamicMaterial) "expression" "(R=1.000000,G=1.000000,B=1.000000,A=1.000000)" :!class /Script/Engine.MaterialInstanceDynamic)
      (Variables|Default|SetopenMouth true))))

(event EventBeginPlay
  (bind _drone (Variables|Default|Getdrone))
  (|CallParentFunction)
  (bind _returnvalue (Rendering|Material|CreateDynamicMaterialInstance _drone 0 "/Game/GameDays/6_4/drone/Drone_MI.Drone_MI" "None" :!class /Script/Engine.PrimitiveComponent))
  (Rendering|Material|SetMaterial _drone 0 _returnvalue)
  (bind _returnvalue_2 (Rendering|Material|CreateDynamicMaterialInstance (Variables|Default|Getman) 0 "/Game/GameDays/6_4/drone/man_hologram2.man_hologram2" "None" :!class /Script/Engine.PrimitiveComponent))
  (Variables|Default|SetdynamicMaterial _returnvalue_2)
  (Utilities|FlowControl|Delay 0.5)
  (if (Utilities|Enum|Equal(Enum) (Variables|Default|GetDroneState) "NewEnumerator0")
    (CallFunction|Play)
    (Rendering|SetActorHiddenInGame false)
    (Default|CallNeedUpdate)
    (else
      (Rendering|SetVisibility (Variables|Default|Getdrone) false false)
      ;[1 1 1] 提示文本
      (Utilities|FlowControl|Delay 5.0)
      (bind _returnvalue_3 (UserInterface|CreateWidget "/Game/GameDays/6_0/HintWidget/Bottom_Hint_Widget.Bottom_Hint_Widget_C"))
      (Rendering|Components|TextRender|SetText (Variables|/Game/GameDays/6_0/HintWidget/Bottom_Hint_Widget.Bottom_Hint_Widget_C|GetTextBlock_79 _returnvalue_3) "一定是哪里在向我传递信息...会是这些闪动的灯牌吗？")
      (Variables|Default|SetBottomHintUI _returnvalue_3)
      (UserInterface|Viewport|AddtoViewport _returnvalue_3 0))))

(event Collision|EventActorBeginOverlap
  (params (OtherActor :type Actor%20Object%20Reference))
  (|CallParentFunction OtherActor) ; This node is disabled and will not be called.\nDrag off pins to build functionality.
)

(event EventTick
  (params (DeltaSeconds :type Float%20%28single-precision%29))
  (bind _returnvalue (Utilities|Time|GetGameTimeinSeconds))
  (bind _returnvalue_2 (* _returnvalue 8.0))
  (bind _returnvalue_3 (Class|KismetMathLibrary|PerlinNoise1D _returnvalue_2))
  (bind _returnvalue_4 (+ _returnvalue_3 0.5))
  (bind _returnvalue_5 (Math|Float|Clamp(Float) _returnvalue_4 0.0 1e+01))
  (bind _returnvalue_6 (/ _returnvalue_5 3.0))
  (|CallParentFunction DeltaSeconds)
  (Utilities|FlowControl|Gate true
    (:Exit
      (Transformation|SetRelativeScale3D (Variables|Default|GetflareRoot) (Math|Vector|MakeVector _returnvalue_6 _returnvalue_6 _returnvalue_6))
      (Rendering|Material|SetVectorParameterValue (Variables|Default|GetdynamicMaterial) "flick" (Utilities|Struct|MakeLinearColor _returnvalue_4 _returnvalue_4 _returnvalue_4 1.0) :!class /Script/Engine.MaterialInstanceDynamic)
      (if (not (Audio|Components|Audio|IsPlaying (Variables|Default|Getspeech)))
        (Utilities|Time|ClearandInvalidateTimerbyHandle (stale Custom|play _returnvalue_7))))))

(fn ConstructionScript
  (|CallParentFunction))

(fn QuitARScene
  (bind _hintui (Variables|Default|GetHintUI))
  (bind _wronghintui (Variables|Default|GetwrongHintUI))
  (Utilities|FlowControl|Sequence
    (:then_0
      (if (Utilities|IsValid _hintui)
        (Widget|RemovefromParent _hintui)))
    (:then_1
      (if (Utilities|IsValid _wronghintui)
        (Widget|RemovefromParent _wronghintui)))
    (:then_2
      (|CallParentFunction))))