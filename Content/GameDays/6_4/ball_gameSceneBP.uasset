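; Scene Blueprint for the AR ball puzzle mission under game day 6_4.
; On EnterScene it spawns the ARBallBuzzle actor at the given transform if no AR scene exists, passing in the IsPassed state and clearing FirstTimeEnter.
; It binds to the puzzle's NeedUpdate event, whose first firing marks the mission completed through a DoOnce.
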(event Custom|update
  ;[1 1 1] 解密，任务完成
  (Utilities|FlowControl|DoOnce false
    (:Completed
      (Variables|Default|SetmissionCompleted true))))

(event EventBeginPlay
  (|CallParentFunction) ; This node is disabled and will not be called.\nDrag off pins to build functionality.
)

(event Collision|EventActorBeginOverlap
  (params (OtherActor :type Actor%20Object%20Reference))
  (|CallParentFunction OtherActor) ; This node is disabled and will not be called.\nDrag off pins to build functionality.
)

(event EventTick
  (params (DeltaSeconds :type Float%20%28single-precision%29))
  (|CallParentFunction DeltaSeconds) ; This node is disabled and will not be called.\nDrag off pins to build functionality.
)

(event EventEnterScene
  (params (transform :type Transform))
  (if (not (Utilities|IsValid (Variables|Default|GetARScene)))
    (Utilities|FlowControl|Sequence
      (:then_0
        (bind _returnvalue (Game|SpawnActorfromClass "/Game/GameDays/6_4/ball/ARBallBuzzle.ARBallBuzzle_C" transform "Undefined" 0 (Variables|Default|GetisPassed) 0))
        ;[1 1 1] 解密，任务完成
        (bind _output_get (Variables|Default|SetARScene _returnvalue))
        (Variables|Default|SetfirstTimeEnter false)
        (EventDispatchers|BindEventtoNeedUpdate _output_get (delegate Custom|update))))))

(fn ConstructionScript
  (|CallParentFunction))