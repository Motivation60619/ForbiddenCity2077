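; Neon background actor that blinks five child light actors in a looping hint sequence, cached as lightActor references on BeginPlay.
; An init phase flashes all lights together, then a hint phase toggles each in numeric order for five timer ticks, leaving it lit.
; Looping timers with counters and FlipFlops drive both phases; after the last light, every light flips off and the cycle restarts.
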(event Custom|initPhase
  ;[1 1 1] 灯的初始闪烁状态
  (Variables|Default|Setcount 0)
  (bind _returnvalue (Utilities|Time|SetTimerbyEvent (delegate Custom|flick) 0.5 true)))

(event Custom|flick
  (bind _lightacttor1 (Variables|Default|GetlightActtor1))
  ;[1 1 1] 灯的初始闪烁状态
  (if (>= (Variables|Default|Getcount) 6)
    (Utilities|Time|ClearandInvalidateTimerbyHandle (stale Custom|initPhase _returnvalue))
    (Utilities|FlowControl|Delay 1.0)
    (CallFunction|HintPhase)
    (else
      (Utilities|FlowControl|Sequence
        (:then_0
          (Utilities|FlowControl|FlipFlop
            (:A
              (Default|Turnon _lightacttor1))
            (:B
              (Default|TurnOff _lightacttor1))))
        (:then_1
          (Math|Integer|IncrementInt (Variables|Default|Getcount)))))))

(event Custom|hintPhase
  ;[1 1 1] 灯的提示状态
  (Variables|Default|Setcount1 0)
  (bind _returnvalue (Utilities|Time|SetTimerbyEvent (delegate Custom|flick2) 0.5 true)))

(event Custom|flick2
  (bind _lightacttor1 (Variables|Default|GetlightActtor1))
  (bind _lightacttor2 (Variables|Default|GetlightActtor2))
  (bind _lightacttor3 (Variables|Default|GetlightActtor3))
  (bind _lightacttor4 (Variables|Default|GetlightActtor4))
  (bind _lightacttor5 (Variables|Default|GetlightActtor5))
  ;[1 1 1] 灯的提示状态
  (if (>= (Variables|Default|Getcount1) 25)
    (Utilities|Time|ClearandInvalidateTimerbyHandle (stale Custom|hintPhase _returnvalue))
    (Utilities|FlowControl|Delay 0.5)
    (Utilities|FlowControl|Sequence
      (:then_0
        (Utilities|FlowControl|FlipFlop :!label _label
          (:A
            (Default|Turnon _lightacttor1))
          (:B
            (Default|TurnOff _lightacttor1))))
      (:then_1
        (Utilities|FlowControl|FlipFlop :!label _label_2
          (:A
            (Default|Turnon _lightacttor3))
          (:B
            (Default|TurnOff _lightacttor3))))
      (:then_2
        (Utilities|FlowControl|FlipFlop :!label _label_3
          (:A
            (Default|Turnon _lightacttor5))
          (:B
            (Default|TurnOff _lightacttor5))))
      (:then_3
        (Utilities|FlowControl|FlipFlop :!label _label_4
          (:A
            (Default|Turnon _lightacttor2))
          (:B
            (Default|TurnOff _lightacttor2))))
      (:then_4
        (Utilities|FlowControl|FlipFlop :!label _label_5
          (:A
            (Default|Turnon _lightacttor4))
          (:B
            (Default|TurnOff _lightacttor4))))
      (:then_5
        (Utilities|FlowControl|Delay 1.0)
        (CallFunction|InitPhase)))
    (else
      (Utilities|FlowControl|Sequence
        (:then_0
          (switch int (/ (Variables|Default|Getcount1) 5)
            (:0
              (goto _label))
            (:1
              (goto _label_4))
            (:2
              (goto _label_2))
            (:3
              (goto _label_5))
            (:4
              (goto _label_3))))
        (:then_1
          (Math|Integer|IncrementInt (Variables|Default|Getcount1)))))))

(event EventBeginPlay
  ;[1 1 1] Comment
  (Utilities|FlowControl|Sequence
    (:then_0
      (Utilities|FlowControl|Sequence
        (:then_0
          (bind _aslight_actor (Utilities|Casting|CastTolightActor (Variables|/Script/Engine.ChildActorComponent|GetChildActor (Variables|Default|Getlight1))))
          (Variables|Default|SetlightActtor1 _aslight_actor))
        (:then_1
          (bind _aslight_actor_2 (Utilities|Casting|CastTolightActor (Variables|/Script/Engine.ChildActorComponent|GetChildActor (Variables|Default|Getlight2))))
          (Variables|Default|SetlightActtor2 _aslight_actor_2))
        (:then_2
          (bind _aslight_actor_3 (Utilities|Casting|CastTolightActor (Variables|/Script/Engine.ChildActorComponent|GetChildActor (Variables|Default|Getlight3))))
          (Variables|Default|SetlightActtor3 _aslight_actor_3))
        (:then_3
          (bind _aslight_actor_4 (Utilities|Casting|CastTolightActor (Variables|/Script/Engine.ChildActorComponent|GetChildActor (Variables|Default|Getlight4))))
          (Variables|Default|SetlightActtor4 _aslight_actor_4))
        (:then_4
          (bind _aslight_actor_5 (Utilities|Casting|CastTolightActor (Variables|/Script/Engine.ChildActorComponent|GetChildActor (Variables|Default|Getlight5))))
          (Variables|Default|SetlightActtor5 _aslight_actor_5))))
    (:then_1
      (CallFunction|InitPhase))))

(event Collision|EventActorBeginOverlap
  (params (OtherActor :type Actor%20Object%20Reference)))

(event EventTick
  (params (DeltaSeconds :type Float%20%28single-precision%29)))

(fn ConstructionScript)