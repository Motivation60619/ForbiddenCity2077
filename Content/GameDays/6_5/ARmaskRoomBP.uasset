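; AR scene actor for a character's room, where the player explores the room UI and finds a mask.
; Construction attaches a gas mask child actor until the mask is taken; BeginPlay shows the room widget, adding hint text on a first visit.
; The closet widget's Getmask event sets the taken flag, swaps the hint, spawns and collects a mask prop, then toggles AR via the pawn.
; QuitARScene cleans up mask and widgets.
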(event Custom|ShutHint
  ;[1 1 1] 当mask还没有被拿走
  (Widget|RemovefromParent (stale EventBeginPlay _returnvalue_4)))

(event Custom|getmask
  ;[1 1 1] 当mask还没有被拿走
  (Variables|Default|SethasMaskBeenTaken? true)
  (Widget|RemovefromParent (Variables|Default|Getroom))
  (bind _returnvalue (UserInterface|CreateWidget "/Game/GameDays/6_0/HintWidget/Bottom_Hint_Widget.Bottom_Hint_Widget_C"))
  (bind _output_get (Variables|Default|SetBottomHint _returnvalue))
  (Rendering|Components|TextRender|SetText (Variables|/Game/GameDays/6_0/HintWidget/Bottom_Hint_Widget.Bottom_Hint_Widget_C|GetTextBlock_79 _output_get) "拿到面具了！虽然不知道有什么用处，不过总比一无所获好")
  (UserInterface|Viewport|AddtoViewport _returnvalue 0)
  (Utilities|FlowControl|Delay 3.0)
  (Actor|DestroyActor (Variables|Default|GetmaskActor))
  (bind _returnvalue_2 (Game|SpawnActorfromClass "/Game/GameDays/6_5/mask_prop.mask_prop_C" (Math|Transform|MakeTransform "0, 0, 0" "0, 0, 0" "3.000000,3.000000,3.000000") "Undefined" 0 0))
  (Default|GotbyPawn _returnvalue_2)
  (Default|CallNeedUpdate)
  (bind _asforbidden_city_pawn (Utilities|Casting|CastToforbiddenCityPawn (Game|Player|GetPlayerPawn 0)))
  (Default|ToggleAREvent (Variables|/Game/core/GameProgressManager.GameProgressManager_C|GetARToggleUI (Variables|/Game/core/forbiddenCityPawn.forbiddenCityPawn_C|GetGameProgressManager _asforbidden_city_pawn))))

(event EventBeginPlay
  (bind _returnvalue (Game|GetPlayerController 0))
  (|CallParentFunction)
  (Utilities|FlowControl|Sequence
    (:then_0
      (if (Variables|Default|GethasMaskBeenTaken?)
        (bind _returnvalue_2 (UserInterface|CreateWidget "/Game/GameDays/6_5/RoomWidget/Room_Widget.Room_Widget_C"))
        (bind _output_get (Variables|Default|Setroom _returnvalue_2))
        (UserInterface|Viewport|AddtoViewport _output_get 0)
        (else
          (Utilities|FlowControl|Sequence
            (:then_0
              ;[1 1 1] 当mask还没有被拿走
              (bind _returnvalue_3 (UserInterface|CreateWidget "/Game/GameDays/6_5/RoomWidget/Room_Widget.Room_Widget_C" _returnvalue))
              (bind _output_get_2 (Variables|Default|Setroom _returnvalue_3))
              (Utilities|FlowControl|Sequence
                (:then_0
                  (UserInterface|Viewport|AddtoViewport _output_get_2 0)
                  (bind _ascloset_widget_1 (Utilities|Casting|CastToCloset_widget1 (Utilities|Array|Get(acopy) (Variables|/Game/GameDays/6_5/RoomWidget/Room_Widget.Room_Widget_C|GetWidgetArray _output_get_2) 2)))
                  (EventDispatchers|BindEventtoGetmask _ascloset_widget_1 (delegate Custom|getmask)))
                (:then_1
                  (EventDispatchers|BindEventtoShutHint _returnvalue_3 (delegate Custom|ShutHint)))))
            (:then_1
              (bind _returnvalue_4 (UserInterface|CreateWidget "/Game/GameDays/6_0/HintWidget/Bottom_Hint_Widget.Bottom_Hint_Widget_C" _returnvalue))
              (Variables|Default|SetBottomHint _returnvalue_4)
              (Rendering|Components|TextRender|SetText (Variables|/Game/GameDays/6_0/HintWidget/Bottom_Hint_Widget.Bottom_Hint_Widget_C|GetTextBlock_79 _returnvalue_4) "这应该就是阿暄的房间，原谅我不请自来，打扰了~这房间好像可以真实地触碰到，那我是不是可以悄悄探索下他的房间呢...")
              (UserInterface|Viewport|AddtoViewport _returnvalue_4 0))))))))

(event Collision|EventActorBeginOverlap
  (params (OtherActor :type Actor%20Object%20Reference))
  (|CallParentFunction OtherActor) ; This node is disabled and will not be called.\nDrag off pins to build functionality.
)

(event EventTick
  (params (DeltaSeconds :type Float%20%28single-precision%29))
  (|CallParentFunction DeltaSeconds) ; This node is disabled and will not be called.\nDrag off pins to build functionality.
)

(fn ConstructionScript
  (|CallParentFunction)
  (if (not (Variables|Default|GethasMaskBeenTaken?))
    (bind _returnvalue (AddComponent|AddChildActorComponent false (Math|Transform|MakeTransform "0, 0,20.000000" "0,90.000000,-90.000000" "0.500000,0.500000,0.500000")))
    (ChildActorComponent|SetChildActorClass _returnvalue "/Game/GameDays/6_5/Mask_Pack/blueprint/BP_GasMask_6.BP_GasMask_6_C")
    (Variables|Default|SetmaskActor (Variables|/Script/Engine.ChildActorComponent|GetChildActor _returnvalue))
    (Variables|Default|Setchild _returnvalue)))

(fn QuitARScene
  (bind _bottomhint (Variables|Default|GetBottomHint))
  (Utilities|FlowControl|Sequence
    (:then_0
      (if (Utilities|IsValid (Variables|Default|GetmaskActor))
        (Actor|DestroyActor (Variables|Default|GetmaskActor))))
    (:then_1
      (if (Utilities|IsValid (Variables|Default|Getroom))
        (Widget|RemovefromParent (Variables|Default|Getroom))))
    (:then_2
      (if (Utilities|IsValid _bottomhint)
        (Widget|RemovefromParent _bottomhint)))
    (:then_3
      (|CallParentFunction))))