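; Game scene Blueprint for the mask room, whose mission completes when the player takes the mask from its AR scene.
; EnterScene spawns the AR mask room actor if none is valid, passing in the saved mask-taken flag, and prints a debug string.
; The room's NeedUpdate event triggers UpdateMaskRoom, which copies the flag back and sets MissionCompleted once the mask is gone.
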(event Custom|updateMaskRoom
  ;[1 1 1] 如果在场景中拿走面具，任务完成
  (bind _asarmask_room_bp (Utilities|Casting|CastToARmaskRoomBP (Variables|Default|GetARScene)))
  (Variables|Default|SethasMaskBeenTaken? (Variables|/Game/GameDays/6_5/ARmaskRoomBP.ARmaskRoomBP_C|GethasMaskBeenTaken? _asarmask_room_bp))
  (if (Variables|/Game/GameDays/6_5/ARmaskRoomBP.ARmaskRoomBP_C|GethasMaskBeenTaken? _asarmask_room_bp)
    (Variables|Default|SetmissionCompleted true)))

(event EventBeginPlay
  (|CallParentFunction) ; This node is disabled and will not be called.\nDrag off pins to build functionality.
)

(event Collision|EventActorBeginOverlap
  (params (OtherActor :type Actor%20Object%20Reference))
  (|CallParentFunction OtherActor) ; This node is disabled and will not be called.\nDrag off pins to build functionality.
)

(event EventTick
  (params (DeltaSeconds :type Float%20%28single-precision%29))
  (|CallParentFunction DeltaSeconds) ; This node is disabled and will not be called.\nDrag off pins to build functionality.
)

(event EventEnterScene
  (params (transform :type Transform))
  (if (not (Utilities|IsValid (Variables|Default|GetARScene)))
    (Utilities|FlowControl|Sequence
      (:then_0
        (bind _returnvalue (Game|SpawnActorfromClass "/Game/GameDays/6_5/ARmaskRoomBP.ARmaskRoomBP_C" transform "Undefined" 0 (Variables|Default|GethasMaskBeenTaken?) false 0))
        (bind _output_get (Variables|Default|SetARScene _returnvalue))
        ;[1 1 1] 如果在场景中拿走面具，任务完成
        (EventDispatchers|BindEventtoNeedUpdate _output_get (delegate Custom|updateMaskRoom)))
      (:then_1
        (Development|PrintString "Hello")))))

(fn ConstructionScript
  (|CallParentFunction))