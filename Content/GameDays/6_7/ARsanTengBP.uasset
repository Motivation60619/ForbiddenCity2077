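; AR SanTeng actor that holds a pen the player can take.
; The construction script adds an enlarged pen mesh while the pen is untaken.
; The gotPen event sets the taken flag, removes the debug UI and mesh, spawns a PenPropObj, calls GotByPawn on it, then CallNeedUpdate.
; The debug UI creation and binding are disconnected, and quitSanTeng is empty.
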(event Custom|gotPen
  ;[1 1 1] 当mask还没有被拿走
  (Variables|Default|SethasPenBeenTaken? true)
  (Widget|RemovefromParent (Variables|Default|GetdebugUI))
  (Components|DestroyComponent (Variables|Default|GetpenComponent))
  (bind _returnvalue (Game|SpawnActorfromClass "/Game/GameDays/6_7/penPropObj.penPropObj_C" (Math|Transform|MakeTransform "0, 0, 0" "0, 0, 0" "3.000000,3.000000,3.000000") "Undefined" 0 0))
  (Default|GotbyPawn _returnvalue)
  (Default|CallNeedUpdate))

(event Custom|quitSanTeng)

(event EventBeginPlay
  (|CallParentFunction))

(event Collision|EventActorBeginOverlap
  (params (OtherActor :type Actor%20Object%20Reference))
  (|CallParentFunction OtherActor) ; This node is disabled and will not be called.\nDrag off pins to build functionality.
)

(event EventTick
  (params (DeltaSeconds :type Float%20%28single-precision%29))
  (|CallParentFunction DeltaSeconds) ; This node is disabled and will not be called.\nDrag off pins to build functionality.
)

(fn ConstructionScript
  (|CallParentFunction)
  (if (not (Variables|Default|GethasPenBeenTaken?))
    (bind _returnvalue (AddComponent|AddStaticMeshComponent false (Math|Transform|MakeTransform "0, 0, 0" "0, 0, 0" "6.000000,6.000000,6.000000")))
    (Components|StaticMesh|SetStaticMesh _returnvalue "/Game/GameDays/6_7/pen.pen")
    (Variables|Default|SetpenComponent _returnvalue)))