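; Game scene Blueprint for SanTeng (game days 6_7) that manages an AR SanTeng actor and its take-the-pen mission.
; On EnterScene it spawns ARsanTengBP at the given transform if none exists, passing in the saved pen-taken state.
; The actor's update event copies that state back and marks the mission completed once the pen is taken.
; QuitScene shuts down and destroys the actor, then calls the parent's quit logic.
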(event Custom|updateSanTeng
  ;[1 1 1] 如果在场景中拿走面具，任务完成
  (bind _output_get (Variables|Default|SethasPenBeenTaken? (Variables|/Game/GameDays/6_7/ARsanTengBP.ARsanTengBP_C|GethasPenBeenTaken? (Variables|Default|GetARSanTeng))))
  (if _output_get
    (Variables|Default|SetmissionCompleted true)))

(event EventBeginPlay
  (|CallParentFunction) ; This node is disabled and will not be called.\nDrag off pins to build functionality.
)

(event Collision|EventActorBeginOverlap
  (params (OtherActor :type Actor%20Object%20Reference))
  (|CallParentFunction OtherActor) ; This node is disabled and will not be called.\nDrag off pins to build functionality.
)

(event EventTick
  (params (DeltaSeconds :type Float%20%28single-precision%29))
  (|CallParentFunction DeltaSeconds) ; This node is disabled and will not be called.\nDrag off pins to build functionality.
)

(event EventEnterScene
  (params (transform :type Transform))
  (if (not (Utilities|IsValid (Variables|Default|GetARSanTeng)))
    (Utilities|FlowControl|Sequence
      (:then_0
        (bind _returnvalue (Game|SpawnActorfromClass "/Game/GameDays/6_7/ARsanTengBP.ARsanTengBP_C" transform "Undefined" 0 (Variables|Default|GethasPenBeenTaken?) 0))
        (bind _output_get (Variables|Default|SetARSanTeng _returnvalue))
        ;[1 1 1] 如果在场景中拿走面具，任务完成
        (EventDispatchers|BindEventtoNeedUpdate _output_get (delegate Custom|updateSanTeng))))))

(event EventQuitScene
  (Utilities|FlowControl|Sequence
    (:then_0
      (if (Utilities|IsValid (Variables|Default|GetARSanTeng))
        (Default|QuitSanTeng (Variables|Default|GetARSanTeng))))
    (:then_2
      (Actor|DestroyActor (Variables|Default|GetARSanTeng)))
    (:then_3
      (|CallParentFunction))))

(fn ConstructionScript
  (|CallParentFunction))