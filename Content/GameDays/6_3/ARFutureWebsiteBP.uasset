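; AR scene Blueprint for the "future website" part of game day 6_3, built around a hologram whose animation can be triggered from a debug UI.
; On BeginPlay it creates the FutureWebsiteDebugUI widget, adds it to the viewport and binds its play event to PlayAnime.
; PlayAnime forwards the call to the BP_Hologram20 child actor.
; QuitARScene removes the widget before running the parent's quit logic.
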(event Custom|PlayAnime
  ;[1 1 1] 谜题还未解开
  (bind _asbp_hologram_20 (Utilities|Casting|CastToBP_Hologram20 (Variables|/Script/Engine.ChildActorComponent|GetChildActor (Variables|Default|GetBP_Hologram20))))
  (Default|CallPlayAnime _asbp_hologram_20))

(event EventBeginPlay
  (|CallParentFunction)
  ;[1 1 1] 谜题还未解开
  (bind _returnvalue (UserInterface|CreateWidget "/Game/GameDays/6_3/futureWebsiteDebugUI.futureWebsiteDebugUI_C"))
  (Variables|Default|SetdebugUI _returnvalue)
  (UserInterface|Viewport|AddtoViewport _returnvalue 0)
  (EventDispatchers|BindEventtoPlayAnime _returnvalue (delegate Custom|PlayAnime)))

(event Collision|EventActorBeginOverlap
  (params (OtherActor :type Actor%20Object%20Reference))
  (|CallParentFunction OtherActor) ; This node is disabled and will not be called.\nDrag off pins to build functionality.
)

(event EventTick
  (params (DeltaSeconds :type Float%20%28single-precision%29))
  ;[1 1 1] 谜题还未解开
  (|CallParentFunction DeltaSeconds) ; This node is disabled and will not be called.\nDrag off pins to build functionality.
)

(fn ConstructionScript
  (|CallParentFunction)
  (if (Variables|Default|GetfondHint)
    _))

(fn QuitARScene
  (bind _debugui (Variables|Default|GetdebugUI))
  (Utilities|FlowControl|Sequence
    (:then_0
      (if (Utilities|IsValid _debugui)
        (Widget|RemovefromParent _debugui)))
    (:then_1
      (|CallParentFunction))))