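; Game scene Blueprint for the day 6_3 "future website" puzzle, which manages its AR scene and mission completion.
; On EnterScene it spawns an ARFutureWebsiteBP at the given transform if none exists, passing in the saved FondHint state and binding to its NeedUpdate event.
; When that event fires, it copies FondHint back from the AR actor and marks the mission completed if the hint is found.
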(event Custom|update
  ;[1 1 1] 解密，任务完成
  (bind _asarfuture_website_bp (Utilities|Casting|CastToARFutureWebsiteBP (Variables|Default|GetARScene)))
  (bind _output_get (Variables|Default|SetfondHint? (Variables|/Game/GameDays/6_3/ARFutureWebsiteBP.ARFutureWebsiteBP_C|GetfondHint _asarfuture_website_bp)))
  (if _output_get
    (Variables|Default|SetmissionCompleted true)))

(event EventBeginPlay
  (|CallParentFunction) ; This node is disabled and will not be called.\nDrag off pins to build functionality.
)

(event Collision|EventActorBeginOverlap
  (params (OtherActor :type Actor%20Object%20Reference))
  (|CallParentFunction OtherActor) ; This node is disabled and will not be called.\nDrag off pins to build functionality.
)

(event EventTick
  (params (DeltaSeconds :type Float%20%28single-precision%29))
  (|CallParentFunction DeltaSeconds) ; This node is disabled and will not be called.\nDrag off pins to build functionality.
)

(event EventEnterScene
  (params (transform :type Transform))
  (if (not (Utilities|IsValid (Variables|Default|GetARScene)))
    (Utilities|FlowControl|Sequence
      (:then_0
        (bind _returnvalue (Game|SpawnActorfromClass "/Game/GameDays/6_3/ARFutureWebsiteBP.ARFutureWebsiteBP_C" transform "Undefined" 0 (Variables|Default|GetfondHint?) false 0))
        (Variables|Default|SetARScene _returnvalue)
        ;[1 1 1] 解密，任务完成
        (EventDispatchers|BindEventtoNeedUpdate (Variables|Default|GetARScene) (delegate Custom|update))))))

(fn ConstructionScript
  (|CallParentFunction))