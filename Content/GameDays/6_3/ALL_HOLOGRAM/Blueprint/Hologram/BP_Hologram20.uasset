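; Hologram display actor that plays a staggered reveal of its panels and continuously spins its HologramBoxLighting component in Tick.
; BeginPlay binds the Play event, which uses a Sequence with separate delays to bring in Main, JumpWin, DYnamic and BG.
; Each panel gets a dynamic material instance whose switch parameter is driven by a timeline.
; DYnamic also animates a begin parameter, with that timeline's Update starting its switch timeline.
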(event Custom|play
  (bind _main (Variables|Default|GetMain))
  (bind _jumpwin (Variables|Default|GetJumpWin))
  (bind _bg (Variables|Default|GetBG))
  (bind _dynamic (Variables|Default|GetDYnamic))
  (Utilities|FlowControl|Sequence
    (:then_0
      ;[1 1 1] 材质加载
      (Utilities|FlowControl|Delay 1.0)
      (bind _returnvalue (Rendering|Material|CreateDynamicMaterialInstance _main 0 "/Game/GameDays/6_3/ALL_HOLOGRAM/Sources/ThirdPersonBP/Blueprints/Textures_Show/MI/MainwinMI.MainwinMI" "switch" :!class /Script/Engine.PrimitiveComponent))
      (Rendering|Material|SetMaterial _main 0 _returnvalue)
      (bind _switch (Timeline|Timeline_2 Play)
        (:Update
          (Rendering|Material|SetScalarParameterValue _returnvalue "switch" _switch :!class /Script/Engine.MaterialInstanceDynamic))))
    (:then_1
      ;;[1 1 1] Description Text
      (Utilities|FlowControl|Delay 2.0)
      (bind _returnvalue_2 (Rendering|Material|CreateDynamicMaterialInstance _jumpwin 0 "/Game/GameDays/6_3/ALL_HOLOGRAM/Sources/ThirdPersonBP/Blueprints/Textures_Show/MI/JumpWinMI.JumpWinMI" "switch" :!class /Script/Engine.PrimitiveComponent))
      (Rendering|Material|SetMaterial _jumpwin 0 _returnvalue_2)
      (bind _switch_2 (Timeline|Timeline_3 Play)
        (:Update
          (Rendering|Material|SetScalarParameterValue _returnvalue_2 "switch" _switch_2 :!class /Script/Engine.MaterialInstanceDynamic))))
    (:then_2
      (Utilities|FlowControl|Delay 4.5)
      (bind _returnvalue_3 (Rendering|Material|CreateDynamicMaterialInstance _bg 0 "/Game/GameDays/6_3/ALL_HOLOGRAM/Sources/ThirdPersonBP/Blueprints/Textures_Show/MI/BGMI.BGMI" "switch" :!class /Script/Engine.PrimitiveComponent))
      (Rendering|Material|SetMaterial _bg 0 _returnvalue_3)
      (bind _switch_3 (Timeline|Timeline_1 Play)
        (:Update
          (Rendering|Material|SetScalarParameterValue _returnvalue_3 "switch" _switch_3 :!class /Script/Engine.MaterialInstanceDynamic))))
    (:then_3
      ;[1 1 1] 动态界面显示
      (Utilities|FlowControl|Delay 4.0)
      (bind _returnvalue_4 (Rendering|Material|CreateDynamicMaterialInstance _dynamic 0 "/Game/GameDays/6_3/ALL_HOLOGRAM/Sources/ThirdPersonBP/Blueprints/Textures_Show/MI/DynamicBegin.DynamicBegin" "switch" :!class /Script/Engine.PrimitiveComponent))
      (Rendering|Material|SetMaterial _dynamic 0 _returnvalue_4)
      (bind _begin (Timeline|Timeline_0 PlayFromStart)
        (:Update
          (Rendering|Material|SetScalarParameterValueonMaterials _dynamic "begin" _begin)
          (bind _switchlight (Timeline|Timeline_4 Play)
            (:Update
              (Rendering|Material|SetScalarParameterValueonMaterials _dynamic "switch" _switchlight))))))))

(event EventBeginPlay
  (EventDispatchers|BindEventtoPlayAnime (delegate Custom|play)))

(event EventTick
  (params (DeltaSeconds :type Float%20%28single-precision%29))
  ;[1 1 1] Building Rotation Animation
  (Transformation|AddRelativeRotation (Variables|Default|GetHologramBoxLighting) (Math|Rotator|MakeRotator 0.0 0.0 (* DeltaSeconds 2e+01)) false false))

(fn ConstructionScript)