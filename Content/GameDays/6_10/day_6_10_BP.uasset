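; Blueprint for game day 6_10, a child day class that supplies that day's content pages and the jump to day 6_11.
; InitMainPages extends the parent by creating a guide widget (passed day "6_4"), a page linked to the "textPuzzle" game scene, and a second page.
; The guide and second page bind next-page events.
; Pressing the finish button calls GoToDay for 6_11, starting from its first page.
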(event Custom|pressFinishButton
  (Default|CallGotoDay "6_11" true))

(event EventBeginPlay
  (|CallParentFunction) ; This node is disabled and will not be called.\nDrag off pins to build functionality.
)

(event Collision|EventActorBeginOverlap
  (params (OtherActor :type Actor%20Object%20Reference))
  (|CallParentFunction OtherActor) ; This node is disabled and will not be called.\nDrag off pins to build functionality.
)

(event EventTick
  (params (DeltaSeconds :type Float%20%28single-precision%29))
  (|CallParentFunction DeltaSeconds) ; This node is disabled and will not be called.\nDrag off pins to build functionality.
)

(fn ConstructionScript
  (|CallParentFunction))

(fn InitMainPages
  (|CallParentFunction)
  (Utilities|FlowControl|Sequence
    (:then_0
      (bind _returnvalue (UserInterface|CreateWidget "/Game/GameDays/6_10/6_10_guidUI.6_10_guidUI_C" 0 "6_4"))
      (Utilities|Array|Add (Variables|Default|GetcontentPages) _returnvalue)
      (EventDispatchers|BindEventtoNextPage _returnvalue (EventDispatchers|CreateEvent :!event NextPage)))
    (:then_1
      (bind _returnvalue_2 (UserInterface|CreateWidget "/Game/GameDays/6_10/6_10_1Page.6_10_1Page_C"))
      (Variables|/Game/GameDays/6_10/6_10_1Page.6_10_1Page_C|SettextPuzzleScene _returnvalue_2 (.Value (Utilities|Map|Find (Variables|Default|GetgameScenes) "textPuzzle")))
      (Utilities|Array|Add (Variables|Default|GetcontentPages) _returnvalue_2))
    (:then_2
      (bind _returnvalue_3 (UserInterface|CreateWidget "/Game/GameDays/6_10/6_10_2Page.6_10_2Page_C"))
      (Utilities|Array|Add (Variables|Default|GetcontentPages) _returnvalue_3)
      (EventDispatchers|BindEventtoNextPage _returnvalue_3 (EventDispatchers|CreateEvent :!event Custom|pressFinishButton)))))