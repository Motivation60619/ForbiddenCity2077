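; Game scene Blueprint for an AR text puzzle that completes its mission when the puzzle is solved.
; On EnterScene it spawns an ARTextPuzzleBP at the given transform if no AR scene exists, passing in the saved solved state.
; It binds to the puzzle's NeedUpdate event, copies the solved flag back and sets MissionCompleted once that is true.
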(event Custom|updateTextPuzzle
  ;[1 1 1] 解密，任务完成
  (bind _asartext_puzzle_bp (Utilities|Casting|CastToARTextPuzzleBP (Variables|Default|GetARScene)))
  (bind _output_get (Variables|Default|SethasPuzzleBeenSolved? (Variables|/Game/GameDays/6_10/ARTextPuzzleBP.ARTextPuzzleBP_C|GetpuzzleHasBeenSolve? _asartext_puzzle_bp)))
  (if _output_get
    (Variables|Default|SetmissionCompleted true)))

(event EventBeginPlay
  (|CallParentFunction) ; This node is disabled and will not be called.\nDrag off pins to build functionality.
)

(event Collision|EventActorBeginOverlap
  (params (OtherActor :type Actor%20Object%20Reference))
  (|CallParentFunction OtherActor) ; This node is disabled and will not be called.\nDrag off pins to build functionality.
)

(event EventTick
  (params (DeltaSeconds :type Float%20%28single-precision%29))
  (|CallParentFunction DeltaSeconds) ; This node is disabled and will not be called.\nDrag off pins to build functionality.
)

(event EventEnterScene
  (params (transform :type Transform))
  (if (not (Utilities|IsValid (Variables|Default|GetARScene)))
    (Utilities|FlowControl|Sequence
      (:then_0
        (bind _returnvalue (Game|SpawnActorfromClass "/Game/GameDays/6_10/ARTextPuzzleBP.ARTextPuzzleBP_C" transform "Undefined" 0 (Variables|Default|GethasPuzzleBeenSolved?) false 0))
        (bind _output_get (Variables|Default|SetARScene _returnvalue))
        ;[1 1 1] 解密，任务完成
        (EventDispatchers|BindEventtoNeedUpdate _output_get (delegate Custom|updateTextPuzzle))))))

(fn ConstructionScript
  (|CallParentFunction))