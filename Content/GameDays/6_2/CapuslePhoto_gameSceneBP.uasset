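; Game scene Blueprint for the capsule photo AR segment under game day 6_2.
; EnterScene spawns the AR capsule photo actor at the supplied transform if no valid instance exists, then clears the IsPassed flag.
; QuitScene destroys that actor before handing off to the parent scene's quit logic.
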(event EventBeginPlay
  (|CallParentFunction))

(event Collision|EventActorBeginOverlap
  (params (OtherActor :type Actor%20Object%20Reference))
  (|CallParentFunction OtherActor) ; This node is disabled and will not be called.\nDrag off pins to build functionality.
)

(event EventTick
  (params (DeltaSeconds :type Float%20%28single-precision%29))
  (|CallParentFunction DeltaSeconds) ; This node is disabled and will not be called.\nDrag off pins to build functionality.
)

(event EventEnterScene
  (params (transform :type Transform))
  (if (not (Utilities|IsValid (Variables|Default|GetARCapsulePhoto)))
    (bind _returnvalue (Game|SpawnActorfromClass "/Game/GameDays/6_2/ARCapuslePhotoBP.ARCapuslePhotoBP_C" transform "Undefined" 0 true 0))
    (Variables|Default|SetARCapsulePhoto _returnvalue)
    (Variables|Default|SetisPassed false)))

(event EventQuitScene
  (bind _arcapsulephoto (Variables|Default|GetARCapsulePhoto))
  (Utilities|FlowControl|Sequence
    (:then_0
      (if (Utilities|IsValid _arcapsulephoto)
        (Actor|DestroyActor _arcapsulephoto)))
    (:then_1
      (|CallParentFunction))))

(fn ConstructionScript
  (|CallParentFunction))