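; AR capsule photo actor that animates a material effect on its Plane in three phases after play begins.
; After a short delay it creates a dynamic instance of CapsulPhot_MI and applies it to the Plane.
; Timelines drive the Begining, Switch and Endpoint scalar parameters in turn.
; Each later timeline is triggered through a Delay wired to the previous timeline's Update output, rather than Finished.
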(event EventBeginPlay
  (bind _plane (Variables|Default|GetPlane))
  (|CallParentFunction)
  (Utilities|FlowControl|Sequence
    (:then_0
      (Utilities|FlowControl|Delay 2.0)
      (bind _returnvalue (Rendering|Material|CreateDynamicMaterialInstance _plane 0 "/Game/GameDays/6_2/material/CapsulPhot_MI.CapsulPhot_MI" "Beginning" :!class /Script/Engine.PrimitiveComponent))
      (Rendering|Material|SetMaterial _plane 0 _returnvalue)
      (bind _begining (Timeline|BeginPlay PlayFromStart)
        (:Update
          (Rendering|Material|SetScalarParameterValueonMaterials _plane "Begining" _begining)
          (Utilities|FlowControl|Delay 2.0)
          (bind _switch (Timeline|switchEffect Play)
            (:Update
              (Rendering|Material|SetScalarParameterValue _returnvalue "Switch" _switch :!class /Script/Engine.MaterialInstanceDynamic)
              (Utilities|FlowControl|Delay 3.5)
              (bind _newtrack_0 (Timeline|EndPoint PlayFromStart)
                (:Update
                  (Rendering|Material|SetScalarParameterValueonMaterials _plane "Endpoint" _newtrack_0))))))))))

(event Collision|EventActorBeginOverlap
  (params (OtherActor :type Actor%20Object%20Reference))
  (|CallParentFunction OtherActor) ; This node is disabled and will not be called.\nDrag off pins to build functionality.
)

(fn ConstructionScript
  (|CallParentFunction))