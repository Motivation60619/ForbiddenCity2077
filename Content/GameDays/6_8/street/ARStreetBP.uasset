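; AR street scene Blueprint for a two-step clue hunt: collect the silver pot, then inspect the wall posters.
; Timelines drive a "switch" parameter on dynamic materials as touch hints.
; Touching the pot spawns and awards Pottery_obj and sets GotPot, which unlocks the poster's wall UI and clue popup.
; Confirming the popup toggles AR off through the pawn's progress manager, while QuitARScene removes the scene's widgets.
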(event Custom|LeaveStreet
  ;[1 1 1] 离开AR场景
  (bind _asforbidden_city_pawn (Utilities|Casting|CastToforbiddenCityPawn (Game|Player|GetPlayerPawn 0)))
  (Default|ToggleAREvent (Variables|/Game/core/GameProgressManager.GameProgressManager_C|GetARToggleUI (Variables|/Game/core/forbiddenCityPawn.forbiddenCityPawn_C|GetGameProgressManager _asforbidden_city_pawn))))

(event EventBeginPlay
  (bind _light (Variables|Default|GetLight))
  (bind _pot (Variables|Default|GetPot))
  (|CallParentFunction)
  (Utilities|FlowControl|Sequence
    (:then_0
      (bind _returnvalue (Rendering|Material|CreateDynamicMaterialInstance _light 0 "/Game/GameDays/6_8/street/material/MI/LightsOnMI.LightsOnMI" "None" :!class /Script/Engine.PrimitiveComponent))
      (Rendering|Material|SetMaterial _light 0 _returnvalue)
      (bind _switch (Timeline|PosterLight PlayFromStart)
        (:Update
          (Rendering|Material|SetScalarParameterValueonMaterials _light "switch" _switch))))
    (:then_1
      (Utilities|FlowControl|Delay 1.0)
      (bind _returnvalue_2 (Rendering|Material|CreateDynamicMaterialInstance _pot 0 "/Game/GameDays/6_8/street/material/MI/PotMI.PotMI" "None" :!class /Script/Engine.PrimitiveComponent))
      (Rendering|Material|SetMaterial _pot 0 _returnvalue_2)
      (bind _newtrack_0 (Timeline|PotHint PlayFromStart)
        (:Update
          (Rendering|Material|SetScalarParameterValueonMaterials _pot "switch" _newtrack_0))))
    (:then_2
      (bind _returnvalue_3 (UserInterface|CreateWidget "/Game/GameDays/6_0/HintWidget/Bottom_Hint_Widget.Bottom_Hint_Widget_C"))
      (Rendering|Components|TextRender|SetText (Variables|/Game/GameDays/6_0/HintWidget/Bottom_Hint_Widget.Bottom_Hint_Widget_C|GetTextBlock_79 _returnvalue_3) "这个器物果然在这里！")
      (Variables|Default|Setbottom_Pop_Up _returnvalue_3)
      (UserInterface|Viewport|AddtoViewport _returnvalue_3 0))))

(event Collision|EventActorBeginOverlap
  (params (OtherActor :type Actor%20Object%20Reference))
  (|CallParentFunction OtherActor) ; This node is disabled and will not be called.\nDrag off pins to build functionality.
)

(event EventSingleTouchedbyPlayer
  (params (component :type Primitive%20Component%20Object%20Reference))
  (bind _light (Variables|Default|GetLight))
  (bind _pot (Variables|Default|GetPot))
  (Development|PrintString (Utilities|String|Append "touch by " (Utilities|GetDisplayName component)))
  (if (== component (Variables|Default|GetBox_poster))
    (if (Variables|Default|Getgot_Pot)
      (Utilities|FlowControl|Sequence
        (:then_0
          (bind _switch (Timeline|PosterLight Stop)
            (:Update
              (Rendering|Material|SetScalarParameterValueonMaterials _light "switch" _switch))))
        (:then_1
          (Rendering|Material|SetMaterial _light 0 "/Engine/Functions/Engine_MaterialFunctions02/ExampleContent/3dParticleOpacity_Mat.3dParticleOpacity_Mat"))
        (:then_2
          (Utilities|FlowControl|DoOnce false
            (:Completed
              (bind _returnvalue (UserInterface|CreateWidget "/Game/GameDays/6_8/street/widget/stree_wallUI.stree_wallUI_C"))
              (Variables|Default|SetStreetWall%20UI _returnvalue)
              (UserInterface|Viewport|AddtoViewport _returnvalue 0)
              (Collision|SetCollisionEnabled (Variables|Default|GetBox_poster) "NoCollision")
              (UserInterface|Animation|PlayAnimation _returnvalue (Variables|/Game/GameDays/6_8/street/widget/stree_wallUI.stree_wallUI_C|GetfadeIn _returnvalue) 0.0 1 "Forward" 1.0 false)
              (Utilities|FlowControl|Sequence
                (:then_0
                  (Default|CallNeedUpdate))))))
        (:then_3
          (bind _returnvalue_2 (UserInterface|CreateWidget "/Game/GameDays/6_0/HintWidget/Pop_Up_Widget.Pop_Up_Widget_C"))
          (Variables|Default|Setpop_Up_Widget _returnvalue_2)
          (Rendering|Components|TextRender|SetText (Variables|/Game/GameDays/6_0/HintWidget/Pop_Up_Widget.Pop_Up_Widget_C|GetTextBlock_PopUp _returnvalue_2) "这两张海报上出现了那几个器物，线索应该就是它们了！但好像还有一个像是盾牌形状的轮廓，会不会又是需要利用那些稀奇古怪的道具呢？ 
点击确定后退出AR")
          (UserInterface|Viewport|AddtoViewport _returnvalue_2 0)
          (EventDispatchers|BindEventtoBacktoPage _returnvalue_2 (delegate Custom|LeaveStreet)))))
    (else
      (Utilities|FlowControl|DoOnce false
        (:Completed
          (Utilities|FlowControl|Sequence
            (:then_0
              (bind _newtrack_0 (Timeline|PotHint Stop)
                (:Update
                  (Rendering|Material|SetScalarParameterValueonMaterials _pot "switch" _newtrack_0))))
            (:then_1
              ;[1 1 1] 得到银壶
              (if (== component (Variables|Default|GetBox_silverPot))
                (Utilities|FlowControl|Sequence
                  (:then_0
                    (Rendering|Material|SetMaterial _pot 0 "/Engine/Functions/Engine_MaterialFunctions02/ExampleContent/3dParticleOpacity_Mat.3dParticleOpacity_Mat"))
                  (:then_1
                    (bind _returnvalue_3 (UserInterface|CreateWidget "/Game/GameDays/6_8/street/widget/silverPotUI.silverPotUI_C"))
                    (Variables|Default|SetSilverPotUi _returnvalue_3)
                    (UserInterface|Viewport|AddtoViewport _returnvalue_3 0)
                    (Collision|SetCollisionEnabled (Variables|Default|GetBox_silverPot) "NoCollision")
                    (Rendering|Material|SetMaterial (Variables|Default|GetPlane) 0 "/Game/GameDays/6_8/street/material/M/Street_EmptyM.Street_EmptyM")
                    (UserInterface|Animation|PlayAnimation _returnvalue_3 (Variables|/Game/GameDays/6_8/street/widget/silverPotUI.silverPotUI_C|GetgetPot _returnvalue_3) 0.0 1 "Forward" 1.0 false)
                    (bind _returnvalue_4 (Game|SpawnActorfromClass "/Game/GameDays/6_8/fourEllementsPuzzle/pottery_obj.pottery_obj_C" (Math|Transform|MakeTransform "0, 0, 0" "0, 0, 0" "1,1,1") "Undefined" 0 0))
                    (Utilities|FlowControl|Sequence
                      (:then_0
                        (bind _returnvalue_5 (UserInterface|CreateWidget "/Game/GameDays/6_0/HintWidget/Bottom_Hint_Widget.Bottom_Hint_Widget_C"))
                        (Variables|Default|Setbottom_Pop_Up _returnvalue_5)
                        (Rendering|Components|TextRender|SetText (Variables|/Game/GameDays/6_0/HintWidget/Bottom_Hint_Widget.Bottom_Hint_Widget_C|GetTextBlock_79 _returnvalue_5) "可是它为什么出现在这儿呢？是想指引我来这里找寻线索么？让我看看，咦，这里的海报好像有什么东西！")
                        (UserInterface|Viewport|AddtoViewport _returnvalue_5 0)
                        (Default|GotbyPawn _returnvalue_4)
                        (Variables|Default|Setgot_Pot true)))))))))))))

(event EventTick
  (params (DeltaSeconds :type Float%20%28single-precision%29)))

(fn ConstructionScript
  (|CallParentFunction))

(fn QuitARScene
  (bind _pop_up_widget (Variables|Default|Getpop_Up_Widget))
  (bind _bottom_pop_up (Variables|Default|Getbottom_Pop_Up))
  (bind _streetwall_ui (Variables|Default|GetStreetWall%20UI))
  (bind _silverpotui (Variables|Default|GetSilverPotUi))
  (Utilities|FlowControl|Sequence
    (:then_0
      (if (Utilities|IsValid _pop_up_widget)
        (Widget|RemovefromParent _pop_up_widget)))
    (:then_1
      (if (Utilities|IsValid _bottom_pop_up)
        (Widget|RemovefromParent _bottom_pop_up)))
    (:then_2
      (if (Utilities|IsValid _streetwall_ui)
        (Widget|RemovefromParent _streetwall_ui)))
    (:then_3
      (if (Utilities|IsValid _silverpotui)
        (Widget|RemovefromParent _silverpotui)))
    (:then_4
      (|CallParentFunction))))