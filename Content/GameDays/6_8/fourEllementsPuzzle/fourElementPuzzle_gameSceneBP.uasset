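; Game scene Blueprint for the four elements puzzle, which launches its AR version and tracks mission completion.
; On EnterScene, if no AR scene exists, it spawns ARFourElementPuzzle with the stored puzzle state, passed flag and whether the pawn's inventory holds the silver pot.
; The AR actor's NeedUpdate event copies its puzzle state back and sets MissionCompleted once that state reaches the solved value.
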(event Custom|CustomEvent_1
  ;[1 1 1] 解密，任务完成
  (bind _asarfour_element_puzzle (Utilities|Casting|CastToARFourElementPuzzle (Variables|Default|GetARScene)))
  (bind _output_get (Variables|Default|SetfourElementsPuzzleState (Variables|/Game/GameDays/6_8/fourEllementsPuzzle/ARFourElementPuzzle.ARFourElementPuzzle_C|GetfourElementsPuzzleState _asarfour_element_puzzle)))
  (if (Utilities|Enum|Equal(Enum) _output_get "NewEnumerator2")
    (Variables|Default|SetmissionCompleted true)))

(event EventBeginPlay
  (|CallParentFunction) ; This node is disabled and will not be called.\nDrag off pins to build functionality.
)

(event Collision|EventActorBeginOverlap
  (params (OtherActor :type Actor%20Object%20Reference))
  (|CallParentFunction OtherActor) ; This node is disabled and will not be called.\nDrag off pins to build functionality.
)

(event EventTick
  (params (DeltaSeconds :type Float%20%28single-precision%29))
  (|CallParentFunction DeltaSeconds) ; This node is disabled and will not be called.\nDrag off pins to build functionality.
)

(event EventEnterScene
  (params (transform :type Transform))
  (if (not (Utilities|IsValid (Variables|Default|GetARScene)))
    (Utilities|FlowControl|Sequence
      (:then_0
        (bind _asforbidden_city_pawn (Utilities|Casting|CastToforbiddenCityPawn (Game|Player|GetPlayerPawn 0)))
        (bind _has (Default|SearchforObj (Variables|/Game/core/forbiddenCityPawn.forbiddenCityPawn_C|GetinventoryActorComponent _asforbidden_city_pawn) "silverPot"))
        (bind _returnvalue (Game|SpawnActorfromClass "/Game/GameDays/6_8/fourEllementsPuzzle/ARFourElementPuzzle.ARFourElementPuzzle_C" transform "Undefined" 0 false (Variables|Default|GetfourElementsPuzzleState) _has (Variables|Default|GetisPassed) 0))
        (bind _output_get (Variables|Default|SetARScene _returnvalue))
        ;[1 1 1] 解密，任务完成
        (EventDispatchers|BindEventtoNeedUpdate _output_get (delegate Custom|CustomEvent_1))))))

(fn ConstructionScript
  (|CallParentFunction))