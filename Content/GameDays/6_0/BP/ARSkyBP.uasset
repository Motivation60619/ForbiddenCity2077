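; ARSkyBP is a sky actor that drives a blend on a plane's Sky_M material, apparently for an AR scene.
; On BeginPlay it creates a dynamic material instance, then either sets blend straight to full if Passed is true or animates it with a timeline.
; When the timeline finishes, it sets Passed and calls NeedUpdate so the change can be picked up elsewhere.
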(event EventBeginPlay
  (|CallParentFunction)
  (bind _returnvalue (Rendering|Material|CreateDynamicMaterialInstance (Variables|Default|GetPlane) 0 "/Game/GameDays/6_0/Material/sky_M.sky_M" "None" :!class /Script/Engine.PrimitiveComponent))
  (Variables|Default|Setsky_M _returnvalue)
  (if (Variables|Default|Getpassed)
    (Rendering|Material|SetScalarParameterValue (Variables|Default|Getsky_M) "blend" 1.0 :!class /Script/Engine.MaterialInstanceDynamic)
    (else
      (bind _newtrack_0 (Timeline|Timeline_0 Play)
        (:Update
          (Rendering|Material|SetScalarParameterValue (Variables|Default|Getsky_M) "blend" _newtrack_0 :!class /Script/Engine.MaterialInstanceDynamic))
        (:Finished
          (Variables|Default|Setpassed true)
          (Default|CallNeedUpdate))))))

(event Collision|EventActorBeginOverlap
  (params (OtherActor :type Actor%20Object%20Reference))
  (|CallParentFunction OtherActor) ; This node is disabled and will not be called.\nDrag off pins to build functionality.
)

(event EventTick
  (params (DeltaSeconds :type Float%20%28single-precision%29))
  (|CallParentFunction DeltaSeconds) ; This node is disabled and will not be called.\nDrag off pins to build functionality.
)

(fn ConstructionScript
  (|CallParentFunction)
  (if (Variables|Default|Getpassed)
    _))