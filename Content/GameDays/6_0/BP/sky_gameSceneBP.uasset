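; Game scene Blueprint for day 6_0 that hosts the AR stone beam puzzle and holds its progress.
; EnterScene spawns ARStoneBeamBP at the given transform if none is valid, seeded with saved hint, phase, first-visit and pass state.
; The puzzle's update event copies back its phase and derives mission completion from it.
; Its hint event records each hint and adds it to the owning 6_0_2Page's hint UI.
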(event Custom|update
  ;[1 1 1] 解密，任务完成
  (bind _asarstone_beam_bp (Utilities|Casting|CastToARStoneBeamBP (Variables|Default|GetARScene)))
  (bind _output_get (Variables|Default|SetStonePuzzlePhase (Variables|/Game/GameDays/6_0/BP/ARStoneBeamBP.ARStoneBeamBP_C|GetStonePuzzlePhase _asarstone_beam_bp)))
  (Variables|Default|SetmissionCompleted (Utilities|Enum|Equal(Enum) _output_get "NewEnumerator4")))

(event Custom|gotHint
  (params (hint :type String))
  (bind _as6_0_2page (Utilities|Casting|CastTo6_0_2Page (Variables|Default|GetownerPager)))
  (Default|AddHint (Variables|/Game/GameDays/6_0/Page_Widget/6_0_2Page.6_0_2Page_C|GethintInfoUI _as6_0_2page) hint)
  (switch string hint
    (:1
      (Variables|Default|SetgotHint1 true))
    (:2
      (Variables|Default|SetgotHint2 true))
    (:3
      (Variables|Default|SetgotHint3 true))))

(event EventBeginPlay
  (|CallParentFunction) ; This node is disabled and will not be called.\nDrag off pins to build functionality.
)

(event Collision|EventActorBeginOverlap
  (params (OtherActor :type Actor%20Object%20Reference))
  (|CallParentFunction OtherActor) ; This node is disabled and will not be called.\nDrag off pins to build functionality.
)

(event EventTick
  (params (DeltaSeconds :type Float%20%28single-precision%29))
  (|CallParentFunction DeltaSeconds) ; This node is disabled and will not be called.\nDrag off pins to build functionality.
)

(event EventEnterScene
  (params (transform :type Transform))
  (bind _stonepuzzlephase (Variables|Default|GetStonePuzzlePhase))
  (if (not (Utilities|IsValid (Variables|Default|GetARScene)))
    (Development|PrintString (Utilities|String|EnumtoString _stonepuzzlephase) true true "(R=1.000000,G=0.007345,B=0.000000,A=1.000000)")
    (bind _returnvalue (Game|SpawnActorfromClass "/Game/GameDays/6_0/BP/ARStoneBeamBP.ARStoneBeamBP_C" transform "Undefined" 0 (Variables|Default|GetgotHint1) (Variables|Default|GetgotHint2) (Variables|Default|GetgotHint3) (Variables|Default|GetpuzzleIsShowed) (Variables|Default|GetfirstTimeEnter) 1 _stonepuzzlephase (Variables|Default|GetisPassed) 0))
    (bind _output_get (Variables|Default|SetARScene _returnvalue))
    ;[1 1 1] 解密，任务完成
    (Variables|Default|SetfirstTimeEnter false)
    (EventDispatchers|BindEventtoNeedUpdate _output_get (delegate Custom|update))
    (EventDispatchers|BindEventtoGotHint _returnvalue (delegate Custom|gotHint))))

(fn ConstructionScript
  (|CallParentFunction))