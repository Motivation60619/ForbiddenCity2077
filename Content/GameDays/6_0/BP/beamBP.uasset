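; Touch-driven stone column puzzle piece that steps up and back down through four heights, one section per touch.
; Timelines slide the scene component vertically with audio, ignoring further touches while animating.
; Each step sets section visibility and capsule size, delayed one second when descending.
; CallUpdatePuzzle runs on each accepted touch without waiting for that delay; single touches also require IsActive.
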(event Custom|touchByPlayer
  (bind _capsule (Variables|Default|GetCapsule))
  (bind _capsule_2 (Variables|Default|GetCapsule))
  (bind _capsule_3 (Variables|Default|GetCapsule))
  (bind _capsule_4 (Variables|Default|GetCapsule))
  (if (not (Variables|Default|GetinAnimationPhase))
    (Utilities|FlowControl|Sequence
      (:then_0
        (if (Variables|Default|GetisIncrease)
          (Variables|Default|SetcurrentVallue (+ (Variables|Default|GetcurrentVallue) 1))
          (CallFunction|AddOneSection)
          (if (== (Variables|Default|GetcurrentVallue) 3)
            (Variables|Default|SetisIncrease false))
          (else
            (Variables|Default|SetcurrentVallue (+ (Variables|Default|GetcurrentVallue) -1))
            (CallFunction|MinusOneSection)
            (if (== (Variables|Default|GetcurrentVallue) 0)
              (Variables|Default|SetisIncrease true))
            (Utilities|FlowControl|Delay 1.0)))
        (switch int (Variables|Default|GetcurrentVallue)
          (:0
            (Development|SetHiddeninGame (Variables|Default|GetStone_Column_F1_Bottom) true true)
            (Components|Capsule|SetCapsuleHalfHeight _capsule_2 26.0 true)
            (Transformation|SetRelativeLocation _capsule_2 "0, 0, 0" false false))
          (:1
            (Development|SetHiddeninGame (Variables|Default|GetStone_Column_F1_Midium) true true)
            (Development|SetHiddeninGame (Variables|Default|GetStone_Column_F1_Top) false true)
            (Components|Capsule|SetCapsuleHalfHeight _capsule_3 4e+01 true)
            (Transformation|SetRelativeLocation _capsule_3 "0, 0,5.300000" false false))
          (:2
            (Development|SetHiddeninGame (Variables|Default|GetStone_Column_F1_Bottom) true true)
            (Development|SetHiddeninGame (Variables|Default|GetStone_Column_F1_Midium) false true)
            (Components|Capsule|SetCapsuleHalfHeight _capsule_4 6e+01 true)
            (Transformation|SetRelativeLocation _capsule_4 "0, 0,9.000000" false false))
          (:3
            (Development|SetHiddeninGame (Variables|Default|GetStone_Column_F1_Bottom) false true)
            (Components|Capsule|SetCapsuleHalfHeight _capsule 8e+01 true)
            (Transformation|SetRelativeLocation _capsule "0, 0,13.000000" false false))))
      (:then_1
        (Default|CallUpdatePuzzle)))))

(event Custom|minusOneSection
  (Variables|Default|SetinAnimationPhase true)
  (Audio|Components|Audio|Play (Variables|Default|GetAudio) 0.0)
  (Variables|Default|SettempZ (.z (Variables|/Script/Engine.SceneComponent|GetRelativeLocation (Variables|Default|GetScene3))))
  (bind _newtrack_0 (Timeline|Timeline_1 PlayFromStart)
    (:Update
      (if (== (Variables|Default|GetcurrentVallue) 2)
        (Transformation|SetRelativeLocation (Variables|Default|GetScene3) (Math|Vector|MakeVector 0.0 0.0 (+ (* _newtrack_0 -4e+01) (Variables|Default|GettempZ))) false false)
        (else
          (Transformation|SetRelativeLocation (Variables|Default|GetScene3) (Math|Vector|MakeVector 0.0 0.0 (+ (* _newtrack_0 -2e+01) (Variables|Default|GettempZ))) false false))))
    (:Finished
      (Variables|Default|SetinAnimationPhase false))))

(event Custom|addOneSection
  (Variables|Default|SetinAnimationPhase true)
  (Audio|Components|Audio|Play (Variables|Default|GetAudio) 0.0)
  (Variables|Default|SettempZ (.z (Variables|/Script/Engine.SceneComponent|GetRelativeLocation (Variables|Default|GetScene3))))
  (bind _newtrack_0 (Timeline|Timeline_0 PlayFromStart)
    (:Update
      (if (== (Variables|Default|GetcurrentVallue) 3)
        (Transformation|SetRelativeLocation (Variables|Default|GetScene3) (Math|Vector|MakeVector 0.0 0.0 (+ (* _newtrack_0 4e+01) (Variables|Default|GettempZ))) false false)
        (else
          (Transformation|SetRelativeLocation (Variables|Default|GetScene3) (Math|Vector|MakeVector 0.0 0.0 (+ (* _newtrack_0 2e+01) (Variables|Default|GettempZ))) false false))))
    (:Finished
      (Variables|Default|SetinAnimationPhase false))))

(event Collision|EventActorBeginOverlap
  (params (OtherActor :type Actor%20Object%20Reference)))

(event EventSingleTouchedbyPlayer
  (params (component :type Primitive%20Component%20Object%20Reference))
  (if (Variables|Default|GetisActive)
    (CallFunction|TouchbyPlayer)))

(event EventTick
  (params (DeltaSeconds :type Float%20%28single-precision%29)))

(fn ConstructionScript)