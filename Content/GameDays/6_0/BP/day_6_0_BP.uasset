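; Day 6_0 game-day Blueprint that handles what happens when a scene of that day is quit.
; Its QuitScene function advances to the next page and marks the scene as passed, only if it has not been passed already.
; The mission-completed and first-time inputs are unused, and the event graph holds only disabled default events.
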(event EventBeginPlay
  (|CallParentFunction) ; This node is disabled and will not be called.\nDrag off pins to build functionality.
)

(event Collision|EventActorBeginOverlap
  (params (OtherActor :type Actor%20Object%20Reference))
  (|CallParentFunction OtherActor) ; This node is disabled and will not be called.\nDrag off pins to build functionality.
)

(event EventTick
  (params (DeltaSeconds :type Float%20%28single-precision%29))
  (|CallParentFunction DeltaSeconds) ; This node is disabled and will not be called.\nDrag off pins to build functionality.
)

(fn ConstructionScript
  (|CallParentFunction))

(fn QuitScene
  (params (missionCompleted :type Boolean) (isFirstTime :type Boolean) (scene :type Game%20Scene%20BP%20Object%20Reference) (isPassed :type Boolean))
  (if (not isPassed)
    (CallFunction|NextPage)
    (Variables|/Game/core/gameSceneBP.gameSceneBP_C|SetisPassed scene true)))