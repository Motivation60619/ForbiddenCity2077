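; AR scene actor for a phased stone-pillar puzzle in a Forbidden City game: find three ridge-beast symbols, then solve a magic-circle puzzle.
; Construction restores the saved phase; touch events collect pulsing hints, reveal the circle and activate the BeamPuzzle child actor.
; That child's click, wrong-click and solved events drive hint widgets, phase updates and completion.
; Pop-ups force exits from AR between phases, and timelines animate dynamic-material glows.
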(event Custom|enterPhase2
  ;[1 1 1] 进入谜题第二部分
  (Utilities|FlowControl|Sequence
    (:then_0
      (bind _returnvalue (UserInterface|CreateWidget "/Game/GameDays/6_0/HintWidget/Bottom_Hint_Widget.Bottom_Hint_Widget_C"))
      (bind _output_get (Variables|Default|SetBottom_Hint_Puzzel _returnvalue))
      (Rendering|Components|TextRender|SetText (Variables|/Game/GameDays/6_0/HintWidget/Bottom_Hint_Widget.Bottom_Hint_Widget_C|GetTextBlock_79 _output_get) "咦，法阵好像有些变化，地面上升起了石柱！（请点击法阵发光处，触发对应机关）")
      (UserInterface|Viewport|AddtoViewport _returnvalue 0))
    (:then_1
      (Development|SetHiddeninGame (Variables|Default|GetlightHint2) true false)
      (Development|SetHiddeninGame (Variables|Default|Getlogo) false false)
      (Collision|SetCollisionEnabled (Variables|Default|GetpuzzleActiveBox) "QueryAndPhysics")
      (Audio|Components|Audio|Play (Variables|Default|GetAudio) 0.0)
      (bind _newtrack_0 (Timeline|Timeline_1 Play)
        (:Update
          (Rendering|Material|SetVectorParameterValue (Variables|Default|GetlogoDynamicMaterial) "intensity" (Utilities|Struct|MakeLinearColor _newtrack_0 _newtrack_0 _newtrack_0 1.0) :!class /Script/Engine.MaterialInstanceDynamic))))))

(event Custom|CustomEvent_0
  (bind _audio (Variables|Default|GetAudio))
  ;[1 1 1] 解决谜题并验证
  (Variables|Default|SetPuzzleSolved true)
  (Audio|Components|Audio|SetSound _audio "/Game/GameDays/6_0/magic.magic")
  (Audio|Components|Audio|Play _audio 0.0)
  (Variables|Default|SetStonePuzzlePhase "NewEnumerator4")
  (Default|CallNeedUpdate))

(event Custom|hintFlick
  (bind _returnvalue (Actor|GetGameTimeSinceCreation))
  (bind _returnvalue_2 (Actor|GetGameTimeSinceCreation))
  (bind _returnvalue_3 (Actor|GetGameTimeSinceCreation))
  (bind _returnvalue_4 (* _returnvalue_2 2.0))
  (bind _returnvalue_5 (+ _returnvalue 711.0))
  (bind _returnvalue_6 (+ _returnvalue_3 1012.0))
  (bind _returnvalue_7 (Math|Trig|Sin(Radians) _returnvalue_4))
  (bind _returnvalue_8 (* _returnvalue_5 2.0))
  (bind _returnvalue_9 (* _returnvalue_6 2.0))
  (bind _returnvalue_10 (Math|Trig|Sin(Radians) _returnvalue_8))
  (bind _returnvalue_11 (Math|Trig|Sin(Radians) _returnvalue_9))
  (bind _returnvalue_12 (+ _returnvalue_7 1.0))
  (bind _returnvalue_13 (/ _returnvalue_12 1.0))
  (bind _returnvalue_14 (+ _returnvalue_10 1.0))
  (bind _returnvalue_15 (+ _returnvalue_11 1.0))
  (bind _returnvalue_16 (/ _returnvalue_14 1.0))
  (bind _returnvalue_17 (/ _returnvalue_15 1.0))
  ;[1 1 1] 提示闪烁
  (Utilities|FlowControl|Gate true) ; enters at Open
)

(event Custom|finishFirstPhase
  ;[1 1 1] 找到所有提示，结束第一部分内容
  (Development|SetHiddeninGame (Variables|Default|GetlightHint2) true false)
  (Development|SetHiddeninGame (Variables|Default|Getlogo) false false)
  (Utilities|FlowControl|Sequence
    (:then_0
      (Audio|Components|Audio|Play (Variables|Default|GetAudio) 0.0)
      (bind _newtrack_0 (Timeline|Timeline_2 Play)
        (:Update
          (Rendering|Material|SetVectorParameterValue (Variables|Default|GetlogoDynamicMaterial) "intensity" (Utilities|Struct|MakeLinearColor _newtrack_0 _newtrack_0 _newtrack_0 1.0) :!class /Script/Engine.MaterialInstanceDynamic))))
    (:then_1
      (Utilities|FlowControl|Delay 2.0)
      (bind _returnvalue (UserInterface|CreateWidget "/Game/GameDays/6_0/HintWidget/Pop_Up_Widget.Pop_Up_Widget_C"))
      (bind _output_get (Variables|Default|SethintWidget _returnvalue))
      (UserInterface|Viewport|AddtoViewport _output_get 0)
      (Rendering|Components|TextRender|SetText (Variables|/Game/GameDays/6_0/HintWidget/Pop_Up_Widget.Pop_Up_Widget_C|GetTextBlock_PopUp _returnvalue) "刚刚那几个脊兽背后好像有些奇怪的符号，我记录了下来，它们会不会是和这个法阵有关系？我先研究下这些脊兽吧。")
      (EventDispatchers|BindEventtoBacktoPage _returnvalue (delegate Custom|Back%20to%20page)))))

(event Custom|FirstTimeClick
  ;[1 1 1] Phase:点击4次后强制退出AR模式
  (if (Utilities|Enum|Equal(Enum) (Variables|Default|GetStonePuzzlePhase) "NewEnumerator1")
    (bind _result (Math|Integer|IncrementInt (Variables|Default|GetclickTimes))
      (:%20%20
        (if (>= _result 3)
          (bind _returnvalue (UserInterface|CreateWidget "/Game/GameDays/6_0/HintWidget/Pop_Up_Widget.Pop_Up_Widget_C"))
          (Rendering|Components|TextRender|SetText (Variables|/Game/GameDays/6_0/HintWidget/Pop_Up_Widget.Pop_Up_Widget_C|GetTextBlock_PopUp _returnvalue) "这么盲目尝试应该也试不出来什么来，一定有什么方向，我想想，应该和那些脊兽背后的符文有关，但是它们是怎么产生关联的呢？看来一定在别处有更多线索... 
点击后退出AR")
          (bind _output_get (Variables|Default|SetPop_Up_Hint _returnvalue))
          (UserInterface|Viewport|AddtoViewport _returnvalue 0)
          (EventDispatchers|BindEventtoBacktoPage _returnvalue (delegate Custom|go%20Next%20Page)))))))

(event Custom|Back%20to%20page
  ;[1 1 1] 找到所有提示，结束第一部分内容
  (Widget|RemovefromParent (stale Custom|finishFirstPhase _returnvalue))
  ;[1 1 1] 强制退出AR模式
  (bind _asforbidden_city_pawn (Utilities|Casting|CastToforbiddenCityPawn (Game|Player|GetPlayerPawn 0)))
  (Default|ToggleAREvent (Variables|/Game/core/GameProgressManager.GameProgressManager_C|GetARToggleUI (Variables|/Game/core/forbiddenCityPawn.forbiddenCityPawn_C|GetGameProgressManager _asforbidden_city_pawn))))

(event Custom|go%20Next%20Page
  ;[1 1 1] Phase:点击4次后强制退出AR模式
  (Variables|Default|SetStonePuzzlePhase "NewEnumerator3")
  (Default|CallNeedUpdate)
  (bind _asforbidden_city_pawn (Utilities|Casting|CastToforbiddenCityPawn (Game|Player|GetPlayerPawn 0)))
  (Default|ToggleAREvent (Variables|/Game/core/GameProgressManager.GameProgressManager_C|GetARToggleUI (Variables|/Game/core/forbiddenCityPawn.forbiddenCityPawn_C|GetGameProgressManager _asforbidden_city_pawn))))

(event Custom|WrongClicked
  (bind _result (Math|Integer|IncrementInt (Variables|Default|GetclickTimes))
    (:%20%20
      (if (>= _result 12)
        (bind _returnvalue (UserInterface|CreateWidget "/Game/GameDays/6_0/HintWidget/Bottom_Hint_Widget.Bottom_Hint_Widget_C"))
        (Rendering|Components|TextRender|SetText (Variables|/Game/GameDays/6_0/HintWidget/Bottom_Hint_Widget.Bottom_Hint_Widget_C|GetTextBlock_79 _returnvalue) "石柱果然和莲花盘以及脊兽的符号有关，看我来破解这个法阵")
        (bind _output_get (Variables|Default|SetBottom_Hint_Puzzel _returnvalue))
        (UserInterface|Viewport|AddtoViewport _returnvalue 0)))))

(event EventBeginPlay
  (|CallParentFunction)
  (Utilities|FlowControl|Sequence
    (:then_0
      (bind _asbeam_puzzle (Utilities|Casting|CastTobeamPuzzle (Variables|/Script/Engine.ChildActorComponent|GetChildActor (Variables|Default|GetbeamPuzzle))))
      (Utilities|FlowControl|Sequence
        (:then_0
          ;[1 1 1] Phase:点击4次后强制退出AR模式
          (EventDispatchers|BindEventtoBeamClicked _asbeam_puzzle (delegate Custom|FirstTimeClick)))
        (:then_1
          (EventDispatchers|BindEventtoWrongClicked _asbeam_puzzle (delegate Custom|WrongClicked)))
        (:then_2
          ;[1 1 1] 解决谜题并验证
          (EventDispatchers|BindEventtoPuzzleSolvedEvent _asbeam_puzzle (delegate Custom|CustomEvent_0)))))
    (:then_1
      (bind _returnvalue (Rendering|Material|CreateDynamicMaterialInstance (Variables|Default|GetBGPlane) 0 0 "None" :!class /Script/Engine.PrimitiveComponent))
      (Variables|Default|SetBGDynamicMaterial _returnvalue)
      (bind _returnvalue_2 (Rendering|Material|CreateDynamicMaterialInstance (Variables|Default|Getlogo) 0 0 "None" :!class /Script/Engine.PrimitiveComponent))
      (Variables|Default|SetlogoDynamicMaterial _returnvalue_2))
    (:then_3
      (bind _newtrack_0 (Timeline|Timeline_0 Play)
        (:Update
          (if (Variables|Default|GetisFirstTime)
            (Rendering|Material|SetScalarParameterValue (Variables|Default|GetBGDynamicMaterial) "opacity" _newtrack_0 :!class /Script/Engine.MaterialInstanceDynamic)
            (else
              (Rendering|Material|SetScalarParameterValue (Variables|Default|GetBGDynamicMaterial) "opacity" 1.0 :!class /Script/Engine.MaterialInstanceDynamic)))
          (Rendering|Material|SetVectorParameterValue (Variables|Default|GetdynamicMaterial1) "intensity" (Utilities|Struct|MakeLinearColor _newtrack_0 _newtrack_0 _newtrack_0 1.0) :!class /Script/Engine.MaterialInstanceDynamic)
          (Rendering|Material|SetVectorParameterValue (Variables|Default|GetdynamicMaterial2) "intensity" (Utilities|Struct|MakeLinearColor _newtrack_0 _newtrack_0 _newtrack_0 1.0) :!class /Script/Engine.MaterialInstanceDynamic)
          (Rendering|Material|SetVectorParameterValue (Variables|Default|GetdynamicMaterial3) "intensity" (Utilities|Struct|MakeLinearColor _newtrack_0 _newtrack_0 _newtrack_0 1.0) :!class /Script/Engine.MaterialInstanceDynamic))))))

(event Collision|EventActorBeginOverlap
  (params (OtherActor :type Actor%20Object%20Reference))
  (|CallParentFunction OtherActor) ; This node is disabled and will not be called.\nDrag off pins to build functionality.
)

(event EventSingleTouchedbyPlayer
  (params (component :type Primitive%20Component%20Object%20Reference))
  (bind _hint1trigger (Variables|Default|Gethint1Trigger))
  (bind _beampuzzle (Variables|Default|GetbeamPuzzle))
  (bind _hint2trigger (Variables|Default|Gethint2Trigger))
  (bind _audio (Variables|Default|GetAudio))
  (bind _hint3trigger (Variables|Default|Gethint3Trigger))
  (bind _puzzleactivebox (Variables|Default|GetpuzzleActiveBox))
  (if (== component (Variables|Default|GetpuzzleActiveBox))
    ;[1 1 1] 激活法阵
    (Development|SetHiddeninGame _beampuzzle false false)
    (bind _asbeam_puzzle (Utilities|Casting|CastTobeamPuzzle (Variables|/Script/Engine.ChildActorComponent|GetChildActor _beampuzzle)))
    (Default|ActivePuzzle _asbeam_puzzle)
    (Development|SetHiddeninGame _puzzleactivebox true false)
    (Utilities|FlowControl|Sequence
      (:then_0
        (bind _returnvalue (UserInterface|CreateWidget "/Game/GameDays/6_0/HintWidget/Bottom_Hint_Widget.Bottom_Hint_Widget_C"))
        (Rendering|Components|TextRender|SetText (Variables|/Game/GameDays/6_0/HintWidget/Bottom_Hint_Widget.Bottom_Hint_Widget_C|GetTextBlock_79 _returnvalue) "这些石柱触碰后可以升起，最多好像只能升起三节，这会是某种机关吗？我来捣鼓一下...（提示：斜视角度体验更佳）")
        (bind _output_get (Variables|Default|SetBottom_Hint_Puzzel _returnvalue))
        (UserInterface|Viewport|AddtoViewport _returnvalue 0))
      (:then_1
        (Collision|SetCollisionEnabled _puzzleactivebox "NoCollision")
        (Variables|Default|SetStonePuzzlePhase "NewEnumerator1")
        (Default|CallNeedUpdate)))
    (elif (== component (Variables|Default|Gethint1Trigger))
      (Collision|SetCollisionEnabled _hint1trigger "NoCollision")
      (Development|SetHiddeninGame _hint1trigger true false)
      (Default|CallGotHint "1")
      (bind _output_get_2 (Variables|Default|SetgetHint1 true))
      ;[1 1 1] 找到所有线索进入第二部分
      (Variables|/Script/Engine.AudioComponent|SetSound _audio 0 :!label _label)
      (Audio|Components|Audio|Play _audio 0.0)
      (if (and (and _output_get_2 (stale _output_get_4)) (stale _output_get_5))
        (Utilities|FlowControl|Delay 1.0)
        (bind _returnvalue_2 (UserInterface|CreateWidget "/Game/GameDays/6_0/HintWidget/Bottom_Hint_Widget.Bottom_Hint_Widget_C"))
        (bind _output_get_3 (Variables|Default|SethintWidget _returnvalue_2))
        (UserInterface|Viewport|AddtoViewport _output_get_3 0)
        (Rendering|Components|TextRender|SetText (Variables|/Game/GameDays/6_0/HintWidget/Bottom_Hint_Widget.Bottom_Hint_Widget_C|GetTextBlock_79 _returnvalue_2) "地面上出现了一个...法阵?")
        (Variables|Default|SetStonePuzzlePhase "NewEnumerator1")
        (Default|CallNeedUpdate)
        (CallFunction|FinishFirstPhase))
      (elif (== component (Variables|Default|Gethint2Trigger))
        (Collision|SetCollisionEnabled _hint2trigger "NoCollision")
        (Development|SetHiddeninGame _hint2trigger true false)
        (Default|CallGotHint "2")
        (bind _output_get_4 (Variables|Default|SetgetHint2 true))
        (goto _label)
        (elif (== component (Variables|Default|Gethint3Trigger))
          (Collision|SetCollisionEnabled _hint3trigger "NoCollision")
          (Development|SetHiddeninGame _hint3trigger true false)
          (Default|CallGotHint "3")
          (bind _output_get_5 (Variables|Default|SetgetHint3 true))
          (goto _label))))))

(event EventTick
  (params (DeltaSeconds :type Float%20%28single-precision%29))
  (bind _returnvalue (Actor|GetGameTimeSinceCreation))
  (bind _returnvalue_2 (Actor|GetGameTimeSinceCreation))
  (bind _returnvalue_3 (Actor|GetGameTimeSinceCreation))
  (bind _returnvalue_4 (* _returnvalue_2 2.0))
  (bind _returnvalue_5 (+ _returnvalue 711.0))
  (bind _returnvalue_6 (+ _returnvalue_3 1012.0))
  (bind _returnvalue_7 (Math|Trig|Sin(Radians) _returnvalue_4))
  (bind _returnvalue_8 (* _returnvalue_5 2.0))
  (bind _returnvalue_9 (* _returnvalue_6 2.0))
  (bind _returnvalue_10 (Math|Trig|Sin(Radians) _returnvalue_8))
  (bind _returnvalue_11 (Math|Trig|Sin(Radians) _returnvalue_9))
  (bind _returnvalue_12 (+ _returnvalue_7 1.0))
  (bind _returnvalue_13 (/ _returnvalue_12 1.0))
  (bind _returnvalue_14 (+ _returnvalue_10 1.0))
  (bind _returnvalue_15 (+ _returnvalue_11 1.0))
  (bind _returnvalue_16 (/ _returnvalue_14 1.0))
  (bind _returnvalue_17 (/ _returnvalue_15 1.0))
  ;[1 1 1] 提示闪烁
  (Utilities|FlowControl|Sequence
    (:then_1
      (Utilities|FlowControl|Gate true
        (:Exit
          (Utilities|FlowControl|Sequence
            (:then_0
              (Rendering|Material|SetVectorParameterValue (Variables|Default|GetdynamicMaterial1) "intensity" (Utilities|Struct|MakeLinearColor _returnvalue_13 _returnvalue_13 _returnvalue_13 1.0) :!class /Script/Engine.MaterialInstanceDynamic))
            (:then_1
              (Rendering|Material|SetVectorParameterValue (Variables|Default|GetdynamicMaterial2) "intensity" (Utilities|Struct|MakeLinearColor _returnvalue_17 _returnvalue_17 _returnvalue_17 1.0) :!class /Script/Engine.MaterialInstanceDynamic))
            (:then_2
              (Rendering|Material|SetVectorParameterValue (Variables|Default|GetdynamicMaterial3) "intensity" (Utilities|Struct|MakeLinearColor _returnvalue_16 _returnvalue_16 _returnvalue_16 1.0) :!class /Script/Engine.MaterialInstanceDynamic))))))))

(fn ConstructionScript
  (bind _hint1trigger (Variables|Default|Gethint1Trigger))
  (bind _beampuzzle (Variables|Default|GetbeamPuzzle))
  (bind _hint2trigger (Variables|Default|Gethint2Trigger))
  (bind _hint3trigger (Variables|Default|Gethint3Trigger))
  (|CallParentFunction)
  (Utilities|FlowControl|Sequence
    (:then_0
      (if (Variables|Default|GetgetHint1)
        (Collision|SetCollisionEnabled _hint1trigger "NoCollision")
        (Development|SetHiddeninGame _hint1trigger true false)))
    (:then_1
      (if (Variables|Default|GetgetHint2)
        (Collision|SetCollisionEnabled _hint2trigger "NoCollision")
        (Development|SetHiddeninGame _hint2trigger true false)))
    (:then_2
      (if (Variables|Default|GetgetHint3)
        (Collision|SetCollisionEnabled _hint3trigger "NoCollision")
        (Development|SetHiddeninGame _hint3trigger true false)))
    (:then_3
      (switch Utilities|FlowControl|Switch|SwitchonStonePuzzlePhace (Variables|Default|GetStonePuzzlePhase)
        (:NewEnumerator0
          (Utilities|FlowControl|Sequence
            (:then_0
              (bind _returnvalue (Rendering|Material|CreateDynamicMaterialInstance (Variables|Default|GetlightHint1) 0 0 "None" :!class /Script/Engine.PrimitiveComponent))
              (Variables|Default|SetdynamicMaterial1 _returnvalue))
            (:then_1
              (bind _returnvalue_2 (Rendering|Material|CreateDynamicMaterialInstance (Variables|Default|GetlightHint2) 0 0 "None" :!class /Script/Engine.PrimitiveComponent))
              (Variables|Default|SetdynamicMaterial2 _returnvalue_2))
            (:then_2
              (bind _returnvalue_3 (Rendering|Material|CreateDynamicMaterialInstance (Variables|Default|GetlightHint3) 0 0 "None" :!class /Script/Engine.PrimitiveComponent))
              (Variables|Default|SetdynamicMaterial3 _returnvalue_3))
            (:then_3
              (CallFunction|HintFlick))))
        (:NewEnumerator1
          (CallFunction|EnterPhase2))
        (:NewEnumerator3
          (Development|SetHiddeninGame (Variables|Default|GetBGPlane) true false)
          (Development|SetHiddeninGame _beampuzzle false false)
          (bind _asbeam_puzzle (Utilities|Casting|CastTobeamPuzzle (Variables|/Script/Engine.ChildActorComponent|GetChildActor _beampuzzle)))
          (Default|ActivePuzzle _asbeam_puzzle))))))

(fn QuitARScene
  (bind _hintwidget (Variables|Default|GethintWidget))
  (bind _bottom_hint_puzzel (Variables|Default|GetBottom_Hint_Puzzel))
  (bind _pop_up_hint (Variables|Default|GetPop_Up_Hint))
  (Utilities|FlowControl|Sequence
    (:then_0
      (if (Utilities|IsValid _hintwidget)
        _
        (else
          _))
      (Widget|RemovefromParent _hintwidget))
    (:then_1
      (if (Utilities|IsValid _bottom_hint_puzzel)
        (Widget|RemovefromParent _bottom_hint_puzzel)))
    (:then_2
      (if (Utilities|IsValid _pop_up_hint)
        (Widget|RemovefromParent _pop_up_hint)))
    (:then_3
      (|CallParentFunction))))