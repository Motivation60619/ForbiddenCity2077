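; AR hologram info actor for game day 6_6 that reveals an island display with three info points when started.
; BeginPlay binds CreateIsland to the start event of the TOUCHToStart widget, which unhides Cube and its children.
; CreateIsland calls ShowText on each DisplayWidgetBP child actor, then writes hardcoded articles and titles into their ARTitleDisplay widgets.
; Only the first point has story text; the others hold placeholder text and URLs.
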(event Custom|createIsland
  ;[1 1 1] 显示极乐岛，标题
  (Development|SetHiddeninGame (Variables|Default|GetCube) false true)
  (Utilities|FlowControl|Sequence
    (:then_1
      (bind _asdisplay_widget_bp (Utilities|Casting|CastToDisplayWidgetBP (Variables|/Script/Engine.ChildActorComponent|GetChildActor (Variables|Default|GetPoint1))))
      (Default|ShowText _asdisplay_widget_bp (Variables|/Game/GameDays/6_6/DisplayWidgetBP.DisplayWidgetBP_C|GetShow_Which_Text _asdisplay_widget_bp)))
    (:then_2
      (bind _asdisplay_widget_bp_2 (Utilities|Casting|CastToDisplayWidgetBP (Variables|/Script/Engine.ChildActorComponent|GetChildActor (Variables|Default|GetPoint2))))
      (Default|ShowText _asdisplay_widget_bp_2 (Variables|/Game/GameDays/6_6/DisplayWidgetBP.DisplayWidgetBP_C|GetShow_Which_Text _asdisplay_widget_bp_2)))
    (:then_3
      (bind _asdisplay_widget_bp_3 (Utilities|Casting|CastToDisplayWidgetBP (Variables|/Script/Engine.ChildActorComponent|GetChildActor (Variables|Default|GetPoint3))))
      (Default|ShowText _asdisplay_widget_bp_3 (Variables|/Game/GameDays/6_6/DisplayWidgetBP.DisplayWidgetBP_C|GetShow_Which_Text _asdisplay_widget_bp_3)))
    (:then_4
      ;[1 1 1] 具体内容编辑
      (Utilities|FlowControl|Sequence
        (:then_0
          (bind _asdisplay_widget_bp_4 (Utilities|Casting|CastToDisplayWidgetBP (Variables|/Script/Engine.ChildActorComponent|GetChildActor (Variables|Default|GetPoint1))))
          (bind _asartitle_display (Utilities|Casting|CastToARTitleDisplay (UserInterface|GetUserWidgetObject (Variables|/Game/GameDays/6_6/DisplayWidgetBP.DisplayWidgetBP_C|GetinfoWidget _asdisplay_widget_bp_4))))
          (Variables|/Game/GameDays/6_6/IslandWidget/ARTitleDisplay.ARTitleDisplay_C|Setarticle _asartitle_display "这天旅行社老板梦伯和雪姑竟然同时缺席，阿暄也没有接到指定工作，于是开始“摸鱼”，先是和爷爷联系询问近况，接着又研究起旅行社内部，对梦伯有了进一步的认知。下午他收到一份来自小说家的快递，里面是一张类似藏宝图的谜图，阿暄起初以为是类似前一天小说家提出那些“神秘传说”，但是无所事事的他仔细看过那张谜图后发现似乎还真的是一张具有指向性的地图，于是阿暄计划次日同小说家一起前往故宫一探究竟。")
          (Variables|/Game/GameDays/6_6/IslandWidget/ARTitleDisplay.ARTitleDisplay_C|SetWebTitle _asartitle_display "项目介绍"))
        (:then_1
          (bind _asdisplay_widget_bp_5 (Utilities|Casting|CastToDisplayWidgetBP (Variables|/Script/Engine.ChildActorComponent|GetChildActor (Variables|Default|GetPoint2))))
          (bind _asartitle_display_2 (Utilities|Casting|CastToARTitleDisplay (UserInterface|GetUserWidgetObject (Variables|/Game/GameDays/6_6/DisplayWidgetBP.DisplayWidgetBP_C|GetinfoWidget _asdisplay_widget_bp_5))))
          (Variables|/Game/GameDays/6_6/IslandWidget/ARTitleDisplay.ARTitleDisplay_C|Setarticle _asartitle_display_2 "Ut enim ad minim veniam, quis nostrud exercitation ullamco laboris nisi ut aliquip ex ea commodo consequat. Duis aute irure dolor in reprehenderit in voluptate velit esse cillum dolore eu fugiat nulla pariatur. Ut enim ad minim veniam, quis nostrud exercitation ullamco laboris nisi ut aliquip ex ea commodo consequat. Duis aute irure dolor in reprehenderit in voluptate velit esse cillum dolore eu fugiat nulla pariatur. Ut enim ad minim veniam, quis nostrud exercitation ullamco laboris nisi ut aliquip ex ea commodo consequat. Duis aute irure dolor in reprehenderit in voluptate velit esse cillum dolore eu fugiat nulla pariatur. ")
          (Variables|/Game/GameDays/6_6/IslandWidget/ARTitleDisplay.ARTitleDisplay_C|SetWebTitle _asartitle_display_2 "http://www.cjodvn.com/zh-2/video/kasjfklnasdg?frompage,,,,,"))
        (:then_2
          (bind _asdisplay_widget_bp_6 (Utilities|Casting|CastToDisplayWidgetBP (Variables|/Script/Engine.ChildActorComponent|GetChildActor (Variables|Default|GetPoint3))))
          (bind _asartitle_display_3 (Utilities|Casting|CastToARTitleDisplay (UserInterface|GetUserWidgetObject (Variables|/Game/GameDays/6_6/DisplayWidgetBP.DisplayWidgetBP_C|GetinfoWidget _asdisplay_widget_bp_6))))
          (Variables|/Game/GameDays/6_6/IslandWidget/ARTitleDisplay.ARTitleDisplay_C|Setarticle _asartitle_display_3 "Excepteur sint occaecat cupidatat non proident, sunt in culpa qui officia deserunt mollit anim id est laborum.Excepteur sint occaecat cupidatat non proident, sunt in culpa qui officia deserunt mollit anim id est laborum.Excepteur sint occaecat cupidatat non proident, sunt in culpa qui officia deserunt mollit anim id est laborum.Excepteur sint occaecat cupidatat non proident, sunt in culpa qui officia deserunt mollit anim id est laborum.")
          (Variables|/Game/GameDays/6_6/IslandWidget/ARTitleDisplay.ARTitleDisplay_C|SetWebTitle _asartitle_display_3 "http://www.cjodvn.com/zh-3/video/kasjfklnasdg?frompage,,,,,"))))))

(event EventBeginPlay
  (|CallParentFunction)
  ;[1 1 1] 点击查看更多
  (bind _asarpressto_display (Utilities|Casting|CastToARPresstoDisplay (UserInterface|GetUserWidgetObject (Variables|Default|GetTOUCHToStart))))
  (EventDispatchers|BindEventtoStartIsland _asarpressto_display (delegate Custom|createIsland)))

(event Collision|EventActorBeginOverlap
  (params (OtherActor :type Actor%20Object%20Reference))
  (|CallParentFunction OtherActor) ; This node is disabled and will not be called.\nDrag off pins to build functionality.
)

(event EventTick
  (params (DeltaSeconds :type Float%20%28single-precision%29))
  (|CallParentFunction DeltaSeconds))

(event EventSingleTouchedbyPlayer
  (params (component :type Primitive%20Component%20Object%20Reference)))

(fn ConstructionScript
  (|CallParentFunction))