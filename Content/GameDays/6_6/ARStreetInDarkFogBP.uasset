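; AR street-in-fog scene actor: the view behind a photo stays blurred by morning miasma until the player uses the filter mask.
; If HasMask is set, BeginPlay binds to the mask's use event, creates a bottom hint about the mask, then immediately runs the mask check.
; That check removes the hint, swaps the plane between clear and blurred materials by BeenUsed, and calls for an update.
; Quitting the AR scene also clears the hint.
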(event Custom|wetherPutMaskOn
  (bind _plane (Variables|Default|GetPlane))
  ;[1 1 1] 戴上面具，视线变清楚
  (Widget|RemovefromParent (stale EventBeginPlay _returnvalue))
  (if (Variables|/Game/core/gamePropObject/propObj.propObj_C|GetbeenUsed (Variables|Default|GetmaskObj))
    (Rendering|Material|SetMaterial _plane 0 "/Game/GameDays/6_8/street/material/M/streetM.streetM")
    (else
      (Rendering|Material|SetMaterial _plane 0 "/Game/GameDays/6_6/streetBlur_M.streetBlur_M")))
  (Default|CallNeedUpdate))

(event Custom|maskBeenUsed?
  (CallFunction|WetherPutMaskon))

(event EventBeginPlay
  (|CallParentFunction)
  (Utilities|FlowControl|Sequence
    (:then_0
      (if (Variables|Default|GethasMask)
        (EventDispatchers|BindEventtoObjBeingUsed (Variables|Default|GetmaskObj) (delegate Custom|maskBeenUsed?))
        (bind _returnvalue (UserInterface|CreateWidget "/Game/GameDays/6_0/HintWidget/Bottom_Hint_Widget.Bottom_Hint_Widget_C"))
        (Variables|Default|SetBottomHint _returnvalue)
        (Rendering|Components|TextRender|SetText (Variables|/Game/GameDays/6_0/HintWidget/Bottom_Hint_Widget.Bottom_Hint_Widget_C|GetTextBlock_79 _returnvalue) "哇，这晨瘴都要蔓延到我面前了！这怎么能够看得清这照片背后的时空呢？对了，之前在阿暄房间内拿到的过滤罩！")
        (UserInterface|Viewport|AddtoViewport _returnvalue 0)
        (CallFunction|WetherPutMaskon)))
    (:then_1
      (Development|PrintString "Hello"))))

(event Collision|EventActorBeginOverlap
  (params (OtherActor :type Actor%20Object%20Reference))
  (|CallParentFunction OtherActor) ; This node is disabled and will not be called.\nDrag off pins to build functionality.
)

(event EventTick
  (params (DeltaSeconds :type Float%20%28single-precision%29))
  (|CallParentFunction DeltaSeconds) ; This node is disabled and will not be called.\nDrag off pins to build functionality.
)

(fn ConstructionScript
  (|CallParentFunction))

(fn QuitARScene
  (bind _bottomhint (Variables|Default|GetBottomHint))
  (Utilities|FlowControl|Sequence
    (:then_0
      (if (Utilities|IsValid _bottomhint)
        (Widget|RemovefromParent _bottomhint)))
    (:then_1
      (|CallParentFunction))))