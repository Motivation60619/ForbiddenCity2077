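; Game-scene Blueprint for the "street in dark fog" AR scene, which spawns the scene and tracks mission completion.
; EnterScene searches the Forbidden City pawn's inventory for "mask" and, if no valid scene exists, spawns ARStreetInDarkFogBP with that result.
; The spawned scene's NeedUpdate is bound to updateMaskRoom, which sets MissionCompleted.
; That branch is hardcoded true, so completion ignores the HasMask value it reads.
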(event Custom|updateMaskRoom
  ;[1 1 1] 如果带mask进入场景，任务完成
  (bind _asarstreet_in_dark_fog_bp (Utilities|Casting|CastToARStreetInDarkFogBP (Variables|Default|GetARScene)))
  (Variables|Default|SethasMask (Variables|/Game/GameDays/6_6/ARStreetInDarkFogBP.ARStreetInDarkFogBP_C|GethasMask _asarstreet_in_dark_fog_bp))
  (if true
    (Variables|Default|SetmissionCompleted true)))

(event EventBeginPlay
  (|CallParentFunction) ; This node is disabled and will not be called.\nDrag off pins to build functionality.
)

(event Collision|EventActorBeginOverlap
  (params (OtherActor :type Actor%20Object%20Reference))
  (|CallParentFunction OtherActor) ; This node is disabled and will not be called.\nDrag off pins to build functionality.
)

(event EventTick
  (params (DeltaSeconds :type Float%20%28single-precision%29))
  (|CallParentFunction DeltaSeconds) ; This node is disabled and will not be called.\nDrag off pins to build functionality.
)

(event EventEnterScene
  (params (transform :type Transform))
  ;[1 1 1] 进入场景时是否有mask
  (bind _asforbidden_city_pawn (Utilities|Casting|CastToforbiddenCityPawn (Game|Player|GetPlayerPawn 0)))
  (bind (_has _obj) (Default|SearchforObj (Variables|/Game/core/forbiddenCityPawn.forbiddenCityPawn_C|GetinventoryActorComponent _asforbidden_city_pawn) "mask"))
  (Variables|Default|SethasMask _has)
  (if (not (Utilities|IsValid (Variables|Default|GetARScene)))
    (Utilities|FlowControl|Sequence
      (:then_0
        (bind _returnvalue (Game|SpawnActorfromClass "/Game/GameDays/6_6/ARStreetInDarkFogBP.ARStreetInDarkFogBP_C" transform "Undefined" 0 (Variables|Default|GethasMask) _obj false 0))
        (bind _output_get (Variables|Default|SetARScene _returnvalue))
        ;[1 1 1] 如果带mask进入场景，任务完成
        (EventDispatchers|BindEventtoNeedUpdate _output_get (delegate Custom|updateMaskRoom))))))

(fn ConstructionScript
  (|CallParentFunction))