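; Scene Blueprint for the hologram info game scene that manages the lifetime of an AR hologram info actor.
; On EnterScene it spawns an ARHoloGraphInfoBP actor and stores the reference, unless a valid one already exists.
; On QuitScene it destroys that actor if valid, then calls the parent quit logic.
; The BeginPlay, overlap and Tick events are disabled stubs.
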(event EventBeginPlay
  (|CallParentFunction) ; This node is disabled and will not be called.\nDrag off pins to build functionality.
)

(event Collision|EventActorBeginOverlap
  (params (OtherActor :type Actor%20Object%20Reference))
  (|CallParentFunction OtherActor) ; This node is disabled and will not be called.\nDrag off pins to build functionality.
)

(event EventTick
  (params (DeltaSeconds :type Float%20%28single-precision%29))
  (|CallParentFunction DeltaSeconds) ; This node is disabled and will not be called.\nDrag off pins to build functionality.
)

(event EventEnterScene
  (params (transform :type Transform))
  (if (not (Utilities|IsValid (Variables|Default|GetARHoloGraphInfo)))
    (Utilities|FlowControl|Sequence
      (:then_0
        (bind _returnvalue (Game|SpawnActorfromClass "/Game/GameDays/6_6/ARHoloGraphInfoBP.ARHoloGraphInfoBP_C" (Math|Transform|MakeTransform "0, 0, 0" "0, 0, 0" "1,1,1") "Undefined" 0 false 0))
        (Variables|Default|SetARHoloGraphInfo _returnvalue)))))

(event EventQuitScene
  (Utilities|FlowControl|Sequence
    (:then_1
      (if (Utilities|IsValid (Variables|Default|GetARHoloGraphInfo))
        (Actor|DestroyActor (Variables|Default|GetARHoloGraphInfo))))
    (:then_2
      (|CallParentFunction))))

(fn ConstructionScript
  (|CallParentFunction))