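; Game scene Blueprint for the 2077City level under GameDays 6_9, which manages that level's AR scene and mission completion.
; On EnterScene it spawns AR2077City at the given transform if no valid ARScene exists, passing in IsPassed to carry over whether it was already cleared.
; It binds the spawned actor's NeedUpdate event to an update handler that sets MissionCompleted once that actor reports IsPassed.
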(event Custom|update
  ;[1 1 1] 解密，任务完成
  (bind _asar2077city (Utilities|Casting|CastToAR2077City (Variables|Default|GetARScene)))
  (if (Variables|/Game/core/gamePropObject/ARScene.ARScene_C|GetisPassed _asar2077city)
    (Variables|Default|SetmissionCompleted true)))

(event EventBeginPlay
  (|CallParentFunction) ; This node is disabled and will not be called.\nDrag off pins to build functionality.
)

(event Collision|EventActorBeginOverlap
  (params (OtherActor :type Actor%20Object%20Reference))
  (|CallParentFunction OtherActor) ; This node is disabled and will not be called.\nDrag off pins to build functionality.
)

(event EventTick
  (params (DeltaSeconds :type Float%20%28single-precision%29))
  (|CallParentFunction DeltaSeconds) ; This node is disabled and will not be called.\nDrag off pins to build functionality.
)

(event EventEnterScene
  (params (transform :type Transform))
  (if (not (Utilities|IsValid (Variables|Default|GetARScene)))
    (Utilities|FlowControl|Sequence
      (:then_0
        (bind _returnvalue (Game|SpawnActorfromClass "/Game/GameDays/6_9/AR2077City.AR2077City_C" transform "Undefined" 0 (Variables|Default|GetisPassed) 0))
        ;[1 1 1] 解密，任务完成
        (bind _output_get (Variables|Default|SetARScene _returnvalue))
        (EventDispatchers|BindEventtoNeedUpdate _output_get (delegate Custom|update))))))

(fn ConstructionScript
  (|CallParentFunction))