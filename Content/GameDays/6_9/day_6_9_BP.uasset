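; Day 6_9 Blueprint that defines that game day's content pages and hands off to day 6_10 when the finish button is pressed.
; InitMainPages extends the parent by creating a guide widget and two page widgets, binding next-page events on the guide and last page.
; The middle page receives the 2077City scene from GameScenes.
; QuitScene advances to the next page and marks the scene passed, only if it was not already passed.
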(event Custom|pressFinishButton
  (Default|CallGotoDay "6_10" true))

(event EventBeginPlay
  (|CallParentFunction) ; This node is disabled and will not be called.\nDrag off pins to build functionality.
)

(event Collision|EventActorBeginOverlap
  (params (OtherActor :type Actor%20Object%20Reference))
  (|CallParentFunction OtherActor) ; This node is disabled and will not be called.\nDrag off pins to build functionality.
)

(event EventTick
  (params (DeltaSeconds :type Float%20%28single-precision%29))
  (|CallParentFunction DeltaSeconds) ; This node is disabled and will not be called.\nDrag off pins to build functionality.
)

(fn ConstructionScript
  (|CallParentFunction))

(fn InitMainPages
  (|CallParentFunction)
  (Utilities|FlowControl|Sequence
    (:then_0
      (bind _returnvalue (UserInterface|CreateWidget "/Game/GameDays/6_9/6_9_guidUI.6_9_guidUI_C" 0 "6_10"))
      (Utilities|Array|Add (Variables|Default|GetcontentPages) _returnvalue)
      (EventDispatchers|BindEventtoNextPage _returnvalue (EventDispatchers|CreateEvent :!event NextPage)))
    (:then_1
      (bind _returnvalue_2 (UserInterface|CreateWidget "/Game/GameDays/6_9/6_9_1Page.6_9_1Page_C"))
      (Variables|/Game/GameDays/6_9/6_9_1Page.6_9_1Page_C|Set2077City _returnvalue_2 (.Value (Utilities|Map|Find (Variables|Default|GetgameScenes) "2077City")))
      (Utilities|Array|Add (Variables|Default|GetcontentPages) _returnvalue_2))
    (:then_2
      (bind _returnvalue_3 (UserInterface|CreateWidget "/Game/GameDays/6_9/6_9_2Page.6_9_2Page_C"))
      (Utilities|Array|Add (Variables|Default|GetcontentPages) _returnvalue_3)
      (EventDispatchers|BindEventtoNextPage _returnvalue_3 (EventDispatchers|CreateEvent :!event Custom|pressFinishButton)))))

(fn QuitScene
  (params (missionCompleted :type Boolean) (isFirstTime :type Boolean) (scene :type Game%20Scene%20BP%20Object%20Reference) (isPassed :type Boolean))
  (if (not isPassed)
    (CallFunction|NextPage)
    (Variables|/Game/core/gameSceneBP.gameSceneBP_C|SetisPassed scene true)))