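; Actor that manages one game day in a Forbidden City game, tracking day state, main page widget and game scenes.
; BeginPlay creates the page widget; day functions advance state, remove the page, or clean scenes and destroy the actor.
; The pawn's GameProgressManager supplies the AR hint UI and save slot name.
; Scene spawning and paging logic are disconnected; load, next-day and scene-return functions are empty stubs.
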(event Custom|updata)

(event EventBeginPlay
  (CallFunction|InitGameScenes)
  (CallFunction|InitMainPages))

(event Collision|EventActorBeginOverlap
  (params (OtherActor :type Actor%20Object%20Reference)))

(event EventTick
  (params (DeltaSeconds :type Float%20%28single-precision%29)))

(fn ConstructionScript)

(fn InitGameScenes
  ;[1 1 1] 创建并初始化当天的所有游戏场景
)

(fn InitMainPages
  (Utilities|FlowControl|Sequence
    (:then_1
      (bind _returnvalue (UserInterface|CreateWidget (Variables|Default|GetmainPageClass)))
      (Variables|Default|SetmainPageOfDay _returnvalue)
      (EventDispatchers|BindEventtoARToggleUIHint (Variables|Default|GetmainPageOfDay) (EventDispatchers|CreateEvent :!event PlayARHintAnim)))))

(fn NextPage
  ;[1 1 1] 进入当天的下一页面
)

(fn EndOfDay
  (Variables|Default|SetgameDayState "NewEnumerator2")
  (Widget|RemovefromParent (Variables|Default|GetmainPageOfDay)))

(fn QuitScene
  (params (missionCompleted :type Boolean) (isFirstTime :type Boolean) (scene :type Game%20Scene%20BP%20Object%20Reference) (isPassed :type Boolean)))

(fn ReturntoDay)

(fn CleanDay
  (Utilities|FlowControl|Sequence
    (:then_0
      (bind _keys (Utilities|Map|Keys (Variables|Default|GetgameScenes)))
      (for _array_element _keys
        (Default|CleanScene (.Value (Utilities|Map|Find (Variables|Default|GetgameScenes) _array_element)))))
    (:then_1
      (Actor|DestroyActor))))

(fn SaveGame
  (bind _asforbidden_city_pawn (Utilities|Casting|CastToforbiddenCityPawn (Game|Player|GetPlayerPawn 0)))
  (bind _returnvalue (SaveGame|CreateSaveGameObject "/Game/core/gameDaySaveObj.gameDaySaveObj_C"))
  (SaveGame|SaveGametoSlot _returnvalue (Variables|/Game/core/GameProgressManager.GameProgressManager_C|GetplayerName (Variables|/Game/core/forbiddenCityPawn.forbiddenCityPawn_C|GetGameProgressManager _asforbidden_city_pawn))))

(fn LoadGame)

(fn PlayARHintAnim
  (bind _asforbidden_city_pawn (Utilities|Casting|CastToforbiddenCityPawn (Game|Player|GetPlayerPawn 0)))
  (UserInterface|Animation|PlayAnimation (Variables|/Game/core/GameProgressManager.GameProgressManager_C|GetARToggleUI (Variables|/Game/core/forbiddenCityPawn.forbiddenCityPawn_C|GetGameProgressManager _asforbidden_city_pawn)) (Variables|/Game/core/UI/copperRingToggleUI.copperRingToggleUI_C|Getanimation_hint (Variables|/Game/core/GameProgressManager.GameProgressManager_C|GetARToggleUI (Variables|/Game/core/forbiddenCityPawn.forbiddenCityPawn_C|GetGameProgressManager _asforbidden_city_pawn))) 0.0 4 "Forward" 1.0 false))

(fn EnterDay
  (params (firstPag :type Boolean))
  (if firstPag
    ;[1 1 1] 从第一页进入这一天
    (if (Utilities|Enum|Equal(Enum) (Variables|Default|GetgameDayState) "NewEnumerator0")
      (Variables|Default|SetgameDayState "NewEnumerator1"))))

(fn NextDay)