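; A game scene actor that manages the lifecycle of an associated AR scene, with an empty enterScene event taking a transform.
; Quitting tells the AR scene to quit, broadcasts a quit event with mission-completed, first-entry and passed flags, then clears the first-entry flag.
; Transform updates are forwarded to the AR scene, and cleanup destroys both actors, with validity checks on the AR scene throughout.
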(event Custom|enterScene
  (params (transform :type Transform)))

(event Custom|quitScene
  ;[1 1 1] 退出场景
  (Utilities|FlowControl|Sequence
    (:then_0
      (if (Utilities|IsValid (Variables|Default|GetARScene))
        (Default|QuitARScene (Variables|Default|GetARScene))))
    (:then_1
      (Default|CallQuitSceneEvent (Variables|Default|GetmissionCompleted) (Variables|Default|GetfirstTimeEnter) self (Variables|Default|GetisPassed)))
    (:then_2
      (Variables|Default|SetfirstTimeEnter false))))

(event EventBeginPlay)

(event Collision|EventActorBeginOverlap
  (params (OtherActor :type Actor%20Object%20Reference)))

(event EventTick
  (params (DeltaSeconds :type Float%20%28single-precision%29)))

(fn ConstructionScript)

(fn CleanScene
  (Utilities|FlowControl|Sequence
    (:then_0
      (if (Utilities|IsValid (Variables|Default|GetARScene))
        (Actor|DestroyActor (Variables|Default|GetARScene))))
    (:then_1
      (Actor|DestroyActor))))

(fn ARUpdateTransform
  (params (transform :type Transform))
  (bind _arscene (Variables|Default|GetARScene))
  (if (Utilities|IsValid _arscene)
    (Default|UpdateTransform _arscene transform)))